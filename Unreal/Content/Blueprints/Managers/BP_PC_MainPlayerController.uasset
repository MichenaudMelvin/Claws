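; Main player controller for a first-person game with a dynamo flashlight, bandage healing, note reading and throwable objects.
; Inputs fire dispatchers that per-feature Bind/Unbind functions connect to handlers, so controls can be toggled individually or all at once.
; Tick line-traces from the camera to highlight interactable items and predicts throw arcs while aiming.
; It also manages draining lamp charge, health, death and pause widgets, and reports noise events for dynamo, healing and death.
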(event EventBeginPlay
  (|SetBP_Player)
  (Variables|Health|SetHealthPoints (Variables|Health|GetMaxHealth))
  (|SetHealthWidget)
  (|SetMenuWidgets)
  (|SetNotesWidget)
  (KeyBindings|BindAll)
  (bind _returnvalue (UserInterface|CreateWidget "/Game/UI/MenuWidgets/WBP_KeyboardBinding.WBP_KeyboardBinding_C"))
  (Variables|Default|SetTEMP_KeyboardBIndingds _returnvalue)
  (Variables|Movement|SetStamina (Variables|Movement|GetMaxStaminaValue)))

(event EventTick
  (params (DeltaSeconds :type Float%20%28single-precision%29))
  (CallFunction|TickInteraction)
  (CallFunction|TickforAiming))

(event Input|ActionEvents|InputActionCrouch
  (params (Key :type Key%20Structure :default "None"))
  ;[1 1 1] Others actions
  (:Pressed
    (Default|CallOnCrouchPressed))
  (:Released
    (Default|CallOnCrouchReleased)))

(event Input|ActionEvents|InputActionPauseGame
  (params (Key :type Key%20Structure :default "None"))
  (bind _pausehud (Variables|UI|GetPauseHUD))
  (:Pressed
    (Utilities|FlowControl|FlipFlop
      (:A
        (Game|SetGamePaused true)
        (UserInterface|Viewport|AddtoViewport _pausehud 0)
        (Variables|Default|SetbShowMouseCursor true))
      (:B
        (Game|SetGamePaused false)
        (Widget|RemovefromParent _pausehud)
        (Variables|Default|SetbShowMouseCursor false)))))

(event Input|ActionEvents|InputActionReloadDynamo
  (params (Key :type Key%20Structure :default "None"))
  ;[1 1 1] Others actions
  (:Pressed
    (Default|CallOnReloadDynamoPressed))
  (:Released
    (Default|CallOnReloadDynamoReleased)))

(event Input|ActionEvents|InputActionDisable/EnableDynamo
  (params (Key :type Key%20Structure :default "None"))
  ;[1 1 1] Others actions
  (:Pressed
    (Default|CallOnDisableEnableDynamo)))

(event Input|ActionEvents|InputActionSprint
  (params (Key :type Key%20Structure :default "None"))
  ;[1 1 1] Movement and camera movement
  (:Pressed
    (Default|CallOnSprintPressed))
  (:Released
    (Default|CallOnSprintReleased)))

(event Input|ActionEvents|InputActionAim
  (params (Key :type Key%20Structure :default "None"))
  ;[1 1 1] Others actions
  (:Pressed
    (Default|CallOnAimPressed))
  (:Released
    (Default|CallOnAimReleased)))

(event Input|ActionEvents|InputActionShoot
  (params (Key :type Key%20Structure :default "None"))
  ;[1 1 1] Others actions
  (:Pressed
    (Default|CallOnShoot)))

(event Input|ActionEvents|InputActionInteract
  (params (Key :type Key%20Structure :default "None"))
  ;[1 1 1] Others actions
  (:Pressed
    (Default|CallOnInteract)))

(event Input|ActionEvents|InputActionHeal
  (params (Key :type Key%20Structure :default "None"))
  ;[1 1 1] Others actions
  (:Pressed
    (Default|CallOnHeal)))

(event Input|AxisEvents|InputAxisTurnKeyboard
  (params (AxisValue :type Float%20%28single-precision%29))
  ;[1 1 1] Movement and camera movement
  (Default|CallOnTurnKeyboard AxisValue))

(event Input|AxisEvents|InputAxisMoveRight
  (params (AxisValue :type Float%20%28single-precision%29))
  ;[1 1 1] Movement and camera movement
  (Default|CallOnMoveRight AxisValue))

(event Input|AxisEvents|InputAxisMoveForward
  (params (AxisValue :type Float%20%28single-precision%29))
  ;[1 1 1] Movement and camera movement
  (Default|CallOnMoveForward AxisValue))

(event Input|AxisEvents|InputAxisLookUpGamepad
  (params (AxisValue :type Float%20%28single-precision%29))
  ;[1 1 1] Movement and camera movement
  (Default|CallOnLookUpGamepad AxisValue))

(event Input|AxisEvents|InputAxisTurnGamepad
  (params (AxisValue :type Float%20%28single-precision%29))
  ;[1 1 1] Movement and camera movement
  (Default|CallOnTurnGamepad AxisValue))

(event Input|AxisEvents|InputAxisLookUpKeyboard
  (params (AxisValue :type Float%20%28single-precision%29))
  ;[1 1 1] Movement and camera movement
  (Default|CallOnLookUpKeyboard AxisValue))

(event Input|KeyboardEvents|K
  (params (Key :type Key%20Structure :default "None"))
  ;[1 0 0] Debug
  (:Pressed
    (Health|TakeDamages 1e+01)))

(event Input|KeyboardEvents|V
  (params (Key :type Key%20Structure :default "None"))
  (bind _temp_keyboardbindingds (Variables|Default|GetTEMP_KeyboardBIndingds))
  ;[1 0 0] Debug
  (:Pressed
    (Utilities|FlowControl|FlipFlop
      (:A
        (UserInterface|Viewport|AddtoViewport _temp_keyboardbindingds 0)
        (Variables|Default|SetbShowMouseCursor true))
      (:B
        (Widget|RemovefromParent _temp_keyboardbindingds)
        (Variables|Default|SetbShowMouseCursor false)))))

(event Custom|TickInteraction
  (bind _bp_player (Variables|Default|GetBP_Player))
  (bind _firstpersoncamera (Variables|/Game/Blueprints/BP_Player.BP_Player_C|GetFirstPersonCamera _bp_player))
  (bind _returnvalue (Transformation|GetWorldLocation _firstpersoncamera))
  (bind (_outhit _returnvalue_2) (Collision|LineTraceByChannel _returnvalue (+ _returnvalue (* (Math|Vector|GetForwardVector _firstpersoncamera) (Variables|Interactions|GetInteractDetectionLenght))) "TraceTypeQuery1" false 0 "None"))
  (if _returnvalue_2
    (bind _asbp_item (Utilities|Casting|CastToBP_Item (.HitActor (Collision|BreakHitResult _outhit)))
      (:then
        (if (not (== _asbp_item (Variables|Items|GetCurrentCheckedItem)))
          (Interactions|UnFeedbackInteraction)
          (bind _output_get (Variables|Items|SetCurrentCheckedItem _asbp_item))
          (Default|FeedbackCanInteract _output_get)))
      (:CastFailed
        (Interactions|UnFeedbackInteraction :!label _label)))
    (else
      (goto _label))))

(event Custom|TickForAiming
  (if (Variables|Items|GetIsAiming)
    (LaunchableObjects|Aim)))

(event Custom|AimPressed
  (Variables|Items|SetIsAiming true)
  (CallFunction|TickforAiming))

(event Custom|AimReleased
  (Variables|Items|SetIsAiming false)
  (bind _asbp_launchable_object (Utilities|Casting|CastToBP_LaunchableObject (Variables|Items|GetItemInHand)))
  (Utilities|Array|Clear (Variables|/Game/Blueprints/LaunchableObjects/BP_LaunchableObject.BP_LaunchableObject_C|GetAimPosition _asbp_launchable_object)))

(event Custom|Shoot
  (bind _asbp_launchable_object (Utilities|Casting|CastToBP_LaunchableObject (Variables|Items|GetItemInHand)))
  (if (Utilities|Array|IsValidIndex (Variables|/Game/Blueprints/LaunchableObjects/BP_LaunchableObject.BP_LaunchableObject_C|GetAimPosition _asbp_launchable_object))
    (Default|Launch _asbp_launchable_object)))

(event Custom|Interact
  (bind _self self)
  (bind _currentcheckeditem (Variables|Items|GetCurrentCheckedItem))
  (bind _returnvalue (Utilities|GetClass _currentcheckeditem))
  (if (UserInterface|Viewport|IsinViewport (Variables|UI|GetNoteHUD))
    (Interactions|StopReadingNote)
    (elif (and (Utilities|IsValid (Variables|Items|GetItemInHand)) (not (Utilities|IsValid (Variables|Items|GetCurrentCheckedItem))))
      (Default|Interact (Variables|Items|GetItemInHand) self)
      (else
        (Utilities|IsValid _currentcheckeditem
          (:Is%20Valid
            (if (and (or (Utilities|ClassIsChildOf _returnvalue "/Game/Blueprints/LaunchableObjects/BP_LaunchableObject.BP_LaunchableObject_C") (== _returnvalue "/Game/Blueprints/LaunchableObjects/BP_LaunchableObject.BP_LaunchableObject_C")) (Utilities|IsValid (Variables|Items|GetItemInHand)))
              (bind _asbp_launchable_object (Utilities|Casting|CastToBP_LaunchableObject (Variables|Items|GetItemInHand)))
              (Default|DropItem _asbp_launchable_object _self true)
              (Default|Interact (Variables|Items|GetCurrentCheckedItem) _self)
              (else
                (Default|Interact (Variables|Items|GetCurrentCheckedItem) self)))))))))

(event Custom|ReloadDynamo
  (bind _bp_player (Variables|Default|GetBP_Player))
  (bind _maxintensity (Variables|Dynamo|GetMaxIntensity))
  (bind _increaseintensityvalue (Variables|Dynamo|GetIncreaseIntensityValue))
  (bind _bp_player_2 (Variables|Default|GetBP_Player))
  (bind _lampedynamo (Variables|/Game/Blueprints/BP_Player.BP_Player_C|GetLampeDynamo _bp_player_2))
  (bind _intensity (Variables|/Script/Engine.LightComponentBase|GetIntensity _lampedynamo))
  (bind _returnvalue (+ _intensity _increaseintensityvalue))
  (bind _returnvalue_2 (Math|Float|Clamp(Float) _returnvalue 0.0 _maxintensity))
  (if (Variables|Dynamo|GetIsReloading)
    ;[1 0.136 0.9612] Reduire la vitesse //// maybe cause des bugs quand crouch
    (Variables|/Script/Engine.CharacterMovementComponent|SetMaxWalkSpeed (Variables|/Script/Engine.Character|GetCharacterMovement _bp_player) (Variables|/Game/Blueprints/BP_Player.BP_Player_C|GetCrouchSpeed _bp_player))
    (Rendering|Components|Light|SetIntensity _lampedynamo _returnvalue_2)
    (Class|AISenseHearing|ReportNoiseEvent (Transformation|GetWorldLocation _lampedynamo) 1.0 (Variables|Default|GetBP_Player) 0.0 "Noise")
    (Utilities|FlowControl|Delay 0.5)
    (if (== _returnvalue_2 (Variables|Dynamo|GetMaxIntensity))
      (CallFunction|StopReload)
      (else
        (CallFunction|ReloadDynamo)))))

(event Custom|StopReload
  (bind _bp_player (Variables|Default|GetBP_Player))
  (bind _lampedynamo (Variables|/Game/Blueprints/BP_Player.BP_Player_C|GetLampeDynamo _bp_player))
  (bind _returnvalue (Transformation|GetWorldLocation _lampedynamo))
  (Variables|Dynamo|SetIsReloading false)
  (CallFunction|ReduceIntensity)
  (Audio|Components|Audio|Stop (Variables|Components|GetAudioReloading))
  (Audio|PlaySoundatLocation "/Game/Sounds/PlayerSounds/S_FinishedRealodingDynamo.S_FinishedRealodingDynamo" _returnvalue "0, 0, 0" 1.0 1.0 0.0 0 0 0)
  (Class|AISenseHearing|ReportNoiseEvent _returnvalue 1.0 _bp_player 0.0 "Noise")
  (Variables|/Script/Engine.CharacterMovementComponent|SetMaxWalkSpeed (Variables|/Script/Engine.Character|GetCharacterMovement _bp_player) (Variables|/Game/Blueprints/BP_Player.BP_Player_C|GetNormalSpeed _bp_player)))

(event Custom|ReloadDynamoPressed
  (Variables|Dynamo|SetIsReloading true)
  (CallFunction|ReloadDynamo)
  (bind _returnvalue (Audio|SpawnSound2D "/Game/Sounds/PlayerSounds/S_ReloadDynamo.S_ReloadDynamo" 1.0 1.0 0.0 0 false false))
  (Variables|Components|SetAudioReloading _returnvalue))

(event Custom|ReduceIntensity
  (bind _bp_player (Variables|Default|GetBP_Player))
  (bind _maxintensity (Variables|Dynamo|GetMaxIntensity))
  (bind _decreaseintensityvalue (Variables|Dynamo|GetDecreaseIntensityValue))
  (bind _lampedynamo (Variables|/Game/Blueprints/BP_Player.BP_Player_C|GetLampeDynamo _bp_player))
  (bind _intensity (Variables|/Script/Engine.LightComponentBase|GetIntensity _lampedynamo))
  (bind _returnvalue (- _intensity _decreaseintensityvalue))
  (bind _returnvalue_2 (Math|Float|Clamp(Float) _returnvalue 0.0 _maxintensity))
  (Rendering|Components|Light|SetIntensity _lampedynamo _returnvalue_2)
  (if (!= _returnvalue_2 0.0)
    (Utilities|FlowControl|Delay 0.1)
    (CallFunction|ReduceIntensity)
    (else
      (Dynamo|Enable/DisableLight))))

(event Custom|ReloadDynamoReleased
  (if (Variables|Dynamo|GetIsReloading)
    (CallFunction|StopReload)))

(event Custom|DisableEnableDynamo
  (bind _bp_player (Variables|Default|GetBP_Player))
  (bind _lampedynamo (Variables|/Game/Blueprints/BP_Player.BP_Player_C|GetLampeDynamo _bp_player))
  (bind _returnvalue (Transformation|GetWorldLocation _lampedynamo))
  (Dynamo|Enable/DisableLight)
  (if (Rendering|IsVisible _lampedynamo)
    (Audio|PlaySoundatLocation "/Game/Sounds/PlayerSounds/S_Dynamo_on.S_Dynamo_on" _returnvalue "0, 0, 0" 1.0 1.0 0.0 0 0 0)
    (else
      (Audio|PlaySoundatLocation "/Game/Sounds/PlayerSounds/S_Dynamo_off.S_Dynamo_off" _returnvalue "0, 0, 0" 1.0 1.0 0.0 0 0 0)))
  (Class|AISenseHearing|ReportNoiseEvent _returnvalue 1.0 (Variables|Default|GetBP_Player) 0.0 "Noise"))

(event Custom|Heal
  (bind _bp_player (Variables|Default|GetBP_Player))
  (bind _returnvalue (Transformation|GetActorLocation _bp_player))
  (if (and (!= (Variables|Health|GetHealthPoints) (Variables|Health|GetMaxHealth)) (> (Variables|Health|GetBandagesNumber) 0))
    (Math|Integer|DecrementInt (Variables|Health|GetBandagesNumber)
      (:%20%20
        (Health|Add/RemoveHealth 2e+01)
        ;[1 0.6891 0] Missing Sound
        (Audio|PlaySoundatLocation 0 _returnvalue "0, 0, 0" 1.0 1.0 0.0 0 0 0)
        (Class|AISenseHearing|ReportNoiseEvent _returnvalue 1.0 _bp_player 0.0 "Noise")
        (Development|PrintString (Utilities|String|Append "Healing" " " (Utilities|String|ToString(Float) (Variables|Health|GetHealthPoints))))
        (Development|PrintString (Utilities|String|Append "Bandages restants : " (Utilities|String|ToString(Integer) (Variables|Health|GetBandagesNumber))))))
    (else
      (Development|PrintString "Pas de bandages ou PV au max"))))

(fn ConstructionScript)

(fn Add/RemoveHealth
  (params (Add%20/%20Remove%20Health :type Float%20%28single-precision%29))
  (bind _bp_player (Variables|Default|GetBP_Player))
  (bind _capsulecomponent (Variables|/Script/Engine.Character|GetCapsuleComponent _bp_player))
  (bind _returnvalue (Transformation|GetRelativeTransform _capsulecomponent))
  (bind _location (Math|Transform|BreakTransform _returnvalue))
  (Variables|Health|SetHealthPoints (Math|Float|Clamp(Float) (+ Add%20/%20Remove%20Health (Variables|Health|GetHealthPoints)) 0.0 (Variables|Health|GetMaxHealth)))
  (if (== (Variables|Health|GetHealthPoints) 0.0)
    ;[1 0.8323 0] Missing Sound
    (Audio|PlaySoundatLocation 0 _location "0, 0, 0" 1.0 1.0 0.0 0 0 0)
    (Class|AISenseHearing|ReportNoiseEvent _location 1.0 (Variables|Default|GetBP_Player) 0.0 "Noise")
    (bind _returnvalue_2 (UserInterface|CreateWidget "/Game/UI/PlayerWidgets/WBP_DeathScreen.WBP_DeathScreen_C"))
    (UserInterface|Viewport|AddtoViewport _returnvalue_2 0)
    (Game|SetGamePaused true)
    (Variables|Default|SetbShowMouseCursor true)))

(fn Enable/DisableLight
  (bind _bp_player (Variables|Default|GetBP_Player))
  (bind _lampedynamo (Variables|/Game/Blueprints/BP_Player.BP_Player_C|GetLampeDynamo _bp_player))
  (Rendering|ToggleVisibility _lampedynamo false)
  (if (Rendering|IsVisible _lampedynamo)
    (CallFunction|ReduceIntensity)))

(fn UnFeedbackInteraction
  (Utilities|IsValid (Variables|Items|GetCurrentCheckedItem)
    (:Is%20Valid
      (Class|BIInteractableObjects|FeedbackStopCanInteract(Message) (Variables|Items|GetCurrentCheckedItem))
      (Variables|Items|SetCurrentCheckedItem 0))))

(fn AddBandages
  (params (Value :type Integer))
  (bind _output_get (Variables|Health|SetBandagesNumber (+ Value (Variables|Health|GetBandagesNumber))))
  (Development|PrintString (Utilities|String|Append "Bandages : " (Utilities|String|ToString(Integer) _output_get))))

(fn Aim
  (bind _bp_player (Variables|Default|GetBP_Player))
  (Utilities|IsValid (Variables|Items|GetItemInHand)
    (:Is%20Valid
      (bind (_outhit _outpathpositions _outlasttracedestination) (Class|GameplayStatics|BlueprintPredictProjectilePathbyTraceChannel (Transformation|GetSocketLocation (Variables|/Game/Blueprints/BP_Player.BP_Player_C|GetMesh2P _bp_player) "hand_r") (* (Math|Vector|GetForwardVector (Variables|/Game/Blueprints/BP_Player.BP_Player_C|GetFirstPersonCamera _bp_player)) (Variables|Items|GetLaunchDistance)) true 1e+01 "ECC_Visibility" true (Utilities|Array|MakeArray _bp_player) "ForOneFrame" 1.0 (Variables|Items|GetLaunchForce)))
      (bind _asbp_launchable_object (Utilities|Casting|CastToBP_LaunchableObject (Variables|Items|GetItemInHand)))
      (bind _output_get (Variables|/Game/Blueprints/LaunchableObjects/BP_LaunchableObject.BP_LaunchableObject_C|SetAimPosition _asbp_launchable_object _outpathpositions))
      (Utilities|Array|Add _output_get _outlasttracedestination))))

(fn TakeDamages
  (params (DamagesTaken :type Float%20%28single-precision%29))
  (bind _healthhud (Variables|Health|GetHealthHUD))
  (Health|Add/RemoveHealth (* -1 DamagesTaken))
  (Interactions|StopReadingNote)
  (if (UserInterface|Viewport|IsinViewport _healthhud)
    (Widget|RemovefromParent (Variables|Health|GetHealthHUD)))
  (UserInterface|Viewport|AddtoViewport _healthhud 0)
  (AddComponent|AddForceFeedbackComponent false)
  ;[1 0.9329 0] TEMP
  (Development|PrintString (Utilities|String|Append "Vie : " (Utilities|String|ToString(Float) (Variables|Health|GetHealthPoints)))))

(fn StopReadingNote
  (Widget|RemovefromParent (Variables|UI|GetNoteHUD))
  (KeyBindings|BindAll))

(fn BindMovement
  (EventDispatchers|BindEventtoOnMoveForward (EventDispatchers|CreateEvent (Variables|Default|GetBP_Player) :!event MoveForward))
  (EventDispatchers|BindEventtoOnMoveRight (EventDispatchers|CreateEvent (Variables|Default|GetBP_Player) :!event MoveRight)))

(fn UnbindMovement
  (EventDispatchers|UnbindallEventsfromOnMoveForward)
  (EventDispatchers|UnbindallEventsfromOnMoveRight))

(fn BindCameraMovement
  (EventDispatchers|BindEventtoOnTurnKeyboard (EventDispatchers|CreateEvent (Variables|Default|GetBP_Player) :!event Turn))
  (EventDispatchers|BindEventtoOnLookUpKeyboard (EventDispatchers|CreateEvent (Variables|Default|GetBP_Player) :!event LookUp))
  (EventDispatchers|BindEventtoOnTurnGamepad (EventDispatchers|CreateEvent (Variables|Default|GetBP_Player) :!event TurnGamepad))
  (EventDispatchers|BindEventtoOnLookUpGamepad (EventDispatchers|CreateEvent (Variables|Default|GetBP_Player) :!event LookUpGamepad)))

(fn UnbindCameraMovement
  (EventDispatchers|UnbindallEventsfromOnTurnKeyboard)
  (EventDispatchers|UnbindallEventsfromOnLookUpKeyboard)
  (EventDispatchers|UnbindallEventsfromOnTurnGamepad)
  (EventDispatchers|UnbindallEventsfromOnLookUpGamepad))

(fn BindDynamo
  (EventDispatchers|BindEventtoOnDisableEnableDynamo (EventDispatchers|CreateEvent :!event Custom|DisableEnableDynamo)))

(fn UnbindDynamo
  (EventDispatchers|UnbindallEventsfromOnDisableEnableDynamo))

(fn BindReloadDynamo
  (EventDispatchers|BindEventtoOnReloadDynamoPressed (EventDispatchers|CreateEvent :!event Custom|ReloadDynamoPressed))
  (EventDispatchers|BindEventtoOnReloadDynamoReleased (EventDispatchers|CreateEvent :!event Custom|ReloadDynamoReleased)))

(fn UnbindReloadDynamo
  (EventDispatchers|UnbindallEventsfromOnReloadDynamoPressed)
  (EventDispatchers|UnbindallEventsfromOnReloadDynamoReleased))

(fn BindSprint
  (EventDispatchers|BindEventtoOnSprintPressed (EventDispatchers|CreateEvent (Variables|Default|GetBP_Player) :!event PressedSprint))
  (EventDispatchers|BindEventtoOnSprintReleased (EventDispatchers|CreateEvent (Variables|Default|GetBP_Player) :!event ReleasedSprint)))

(fn UnbindSprint
  (EventDispatchers|UnbindallEventsfromOnSprintPressed)
  (EventDispatchers|UnbindallEventsfromOnSprintReleased))

(fn BindAim
  (EventDispatchers|BindEventtoOnAimPressed (EventDispatchers|CreateEvent :!event Custom|AimPressed))
  (EventDispatchers|BindEventtoOnAimReleased (EventDispatchers|CreateEvent :!event Custom|AimReleased)))

(fn UnbindAim
  (EventDispatchers|UnbindallEventsfromOnAimPressed)
  (EventDispatchers|UnbindallEventsfromOnAimReleased))

(fn BindShoot
  (EventDispatchers|BindEventtoOnShoot (EventDispatchers|CreateEvent :!event Custom|Shoot)))

(fn UnbindShoot
  (EventDispatchers|UnbindallEventsfromOnShoot))

(fn BindInteract
  (EventDispatchers|BindEventtoOnInteract (EventDispatchers|CreateEvent :!event Custom|Interact)))

(fn UnbindInteract
  (EventDispatchers|UnbindallEventsfromOnInteract))

(fn BindHeal
  (EventDispatchers|BindEventtoOnHeal (EventDispatchers|CreateEvent :!event Custom|Heal)))

(fn UnbindHeal
  (EventDispatchers|UnbindallEventsfromOnHeal))

(fn BindCrouch
  (EventDispatchers|BindEventtoOnCrouchPressed (EventDispatchers|CreateEvent (Variables|Default|GetBP_Player) :!event CrouchPressed))
  (EventDispatchers|BindEventtoOnCrouchReleased (EventDispatchers|CreateEvent (Variables|Default|GetBP_Player) :!event CrouchReleased)))

(fn UnbindCrouch
  (EventDispatchers|UnbindallEventsfromOnCrouchPressed)
  (EventDispatchers|UnbindallEventsfromOnCrouchReleased))

(fn BindAll
  (KeyBindings|UnbindAll)
  (KeyBindings|BindMovement)
  (KeyBindings|BindCameraMovement)
  (KeyBindings|BindSprint)
  (KeyBindings|BindDynamo)
  (KeyBindings|BindReloadDynamo)
  (KeyBindings|BindAim)
  (KeyBindings|BindShoot)
  (KeyBindings|BindInteract)
  (KeyBindings|BindHeal)
  (KeyBindings|BindCrouch))

(fn UnbindAll
  (KeyBindings|UnbindMovement)
  (KeyBindings|UnbindCameraMovement)
  (KeyBindings|UnbindSprint)
  (KeyBindings|UnbindDynamo)
  (KeyBindings|UnbindReloadDynamo)
  (KeyBindings|UnbindAim)
  (KeyBindings|UnbindShoot)
  (KeyBindings|UnbindInteract)
  (KeyBindings|UnbindHeal)
  (KeyBindings|UnbindCrouch))