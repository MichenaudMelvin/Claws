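; Throwable pickup that the player carries and launches along aimed points, making noise where it lands.
; Interact attaches it to the player's Mesh2P and registers it as ItemInHand, hiding the interact feedback while held.
; Launch clears the hand, then a timeline lerps the actor through each AimPosition point in turn.
; After the last point it clears the path, detaches, plays a sound and reports a noise event.
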(event Custom|LaunchTimeline
  (bind _staticmesh (Variables|Default|GetStaticMesh))
  (bind _returnvalue (Transformation|GetWorldLocation _staticmesh))
  (bind _launch (Timeline|LaunchTimeline_ Play)
    (:Update
      (Transformation|SetActorLocation (Math|Vector|Lerp(Vector) (Transformation|GetActorLocation) (Utilities|Array|Get(acopy) (Variables|Aiming|GetAimPosition) (Variables|Aiming|GetIndexPosition)) _launch) false false))
    (:Finished
      (if (== (- (Utilities|Array|Length (Variables|Aiming|GetAimPosition)) 1) (Variables|Aiming|GetIndexPosition))
        (Utilities|Array|Clear (Variables|Aiming|GetAimPosition))
        (Transformation|DetachFromActor "KeepRelative" "KeepRelative" "KeepRelative")
        (Audio|PlaySoundatLocation 0 _returnvalue "0, 0, 0" 1.0 1.0 0.0 0 0 0)
        (Class|AISenseHearing|ReportNoiseEvent _returnvalue 1.0 self 0.0 "Noise")
        (else
          (Math|Integer|IncrementInt (Variables|Aiming|GetIndexPosition)
            (:%20%20
              (CallFunction|LaunchTimeline))))))))

(event EventFeedbackCanInteract
  (if (not (Variables|Aiming|GetInHandOfPlayer))
    (|CallParentFunction)))

(event EventInteract
  (params (MainPlayerController :type BP%20PC%20Main%20Player%20Controller%20Object%20Reference))
  (|CallParentFunction MainPlayerController)
  (Variables|/Game/Blueprints/Managers/BP_PC_MainPlayerController.BP_PC_MainPlayerController_C|SetItemInHand MainPlayerController self)
  (CallFunction|FeedbackStopCanInteract)
  (Variables|Aiming|SetInHandOfPlayer true)
  (Transformation|AttachComponentToComponent (Variables|/Game/Blueprints/BP_Player.BP_Player_C|GetMesh2P (Variables|/Game/Blueprints/Managers/BP_PC_MainPlayerController.BP_PC_MainPlayerController_C|GetBP_Player MainPlayerController)) "None" "KeepWorld" "KeepWorld" "KeepWorld" true))

(fn ConstructionScript
  (|CallParentFunction)
  (Components|StaticMesh|SetStaticMesh (Variables|Default|GetStaticMesh) (Variables|Default|GetObjectMesh)))

(fn Launch
  (if (and (Variables|Aiming|GetInHandOfPlayer) (== (Components|Timeline|GetPlaybackPosition (Variables|Default|GetLaunchTimeline_)) 0.0))
    (Variables|Aiming|SetInHandOfPlayer false)
    (Variables|/Game/Blueprints/Managers/BP_PC_MainPlayerController.BP_PC_MainPlayerController_C|SetItemInHand (CallFunction|CallMainPlayerController) 0)
    (Variables|Aiming|SetIndexPosition 0)
    (Components|Timeline|SetPlaybackPosition (Variables|Default|GetLaunchTimeline_) 0.0 false true)
    (CallFunction|LaunchTimeline)))