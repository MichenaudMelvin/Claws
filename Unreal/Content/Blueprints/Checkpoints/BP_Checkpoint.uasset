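; A checkpoint actor that saves the game when the player overlaps it.
; It becomes the player controller's current checkpoint only if none is set or its ID is higher, so progress never moves backward.
; Saving writes the checkpoint's location, notes inventory and held item into a new BP_SavedData object, then saves it asynchronously to its slot, logging the result.
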(event Custom|SaveGame
  (bind _mainplayercontroller (CallFunction|CallMainPlayerController))
  (bind _returnvalue (SaveGame|CreateSaveGameObject "/Game/Blueprints/Checkpoints/BP_SavedData.BP_SavedData_C"))
  (bind _output_get (Variables|Default|SetSaveGameInstance _returnvalue))
  (Variables|/Game/Blueprints/Checkpoints/BP_SavedData.BP_SavedData_C|SetPlayerLocation _output_get (Transformation|GetActorLocation self))
  (Variables|/Game/Blueprints/Checkpoints/BP_SavedData.BP_SavedData_C|SetPlayerNotesInventory (Variables|Default|GetSaveGameInstance) (Variables|/Game/Blueprints/Managers/BP_PC_MainPlayerController.BP_PC_MainPlayerController_C|GetNotesInventory _mainplayercontroller))
  (Variables|/Game/Blueprints/Checkpoints/BP_SavedData.BP_SavedData_C|SetPlayerItem (Variables|Default|GetSaveGameInstance) (Variables|/Game/Blueprints/Managers/BP_PC_MainPlayerController.BP_PC_MainPlayerController_C|GetItemInHand _mainplayercontroller))
  (bind _bsuccess (|AsyncSaveGametoSlot (Variables|Default|GetSaveGameInstance) (Variables|/Game/Blueprints/Checkpoints/BP_SavedData.BP_SavedData_C|GetSlotName (Variables|Default|GetSaveGameInstance)) (Variables|/Game/Blueprints/Checkpoints/BP_SavedData.BP_SavedData_C|GetUserIndex (Variables|Default|GetSaveGameInstance)))
    (:then
      (Development|PrintString "Saving..." false true "(R=0.000000,G=0.660000,B=1.000000,A=1.000000)" 0.0))
    (:Completed
      (if _bsuccess
        (Development|PrintString "Saved" false true "(R=0.000000,G=0.660000,B=1.000000,A=1.000000)" 0.0)
        (else
          (Development|PrintString "Save failled" false true "(R=0.000000,G=0.660000,B=1.000000,A=1.000000)" 0.0))))))

(event Collision|EventActorBeginOverlap
  (params (OtherActor :type Actor%20Object%20Reference))
  (bind _mainplayercontroller (CallFunction|CallMainPlayerController))
  (Utilities|CheckTargetClass OtherActor "/Game/Blueprints/BP_Player.BP_Player_C"
    (:true
      (Utilities|IsValid (Variables|/Game/Blueprints/Managers/BP_PC_MainPlayerController.BP_PC_MainPlayerController_C|GetCurrentCheckpoint _mainplayercontroller)
        (:Is%20Valid
          (if (> (Variables|Default|GetID) (Variables|BP_Checkpoint_C|GetID (Variables|/Game/Blueprints/Managers/BP_PC_MainPlayerController.BP_PC_MainPlayerController_C|GetCurrentCheckpoint _mainplayercontroller)))
            (Variables|/Game/Blueprints/Managers/BP_PC_MainPlayerController.BP_PC_MainPlayerController_C|SetCurrentCheckpoint _mainplayercontroller self)
            (CallFunction|SaveGame)))
        (:Is%20Not%20Valid
          (Variables|/Game/Blueprints/Managers/BP_PC_MainPlayerController.BP_PC_MainPlayerController_C|SetCurrentCheckpoint _mainplayercontroller self)
          (CallFunction|SaveGame))))))

(fn ConstructionScript
  (|CallParentFunction))