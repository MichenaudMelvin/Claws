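; Garage door Blueprint, derived from an interactable parent, that opens once with a warning beacon and makes the Button its interaction target.
; OpenandCloseDoor lights two spotlights that Tick spins while active, then after a delay triggers AI-audible noise and plays the slowed door animation.
; The lights and spin switch off after a timed wait.
; A helper macro checks whether the linked Generator is enabled, but the event graph shown never calls it.
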(event EventBeginPlay
  (bind _targetinteraction (Variables|Default|GetTargetInteraction))
  (Utilities|Array|Add _targetinteraction (Variables|Default|GetButton))
  (Utilities|Array|RemoveItem _targetinteraction (Variables|Default|GetStaticMesh))
  (|CallParentFunction)
  (Audio|Components|Audio|Stop (Variables|Default|GetGarageAudioSource))
  (Variables|Default|SetInitialIntensity (Variables|/Script/Engine.LightComponentBase|GetIntensity (Variables|Default|GetSpotLightUP)))
  (CallFunction|SetLightsIntensity 0.0))

(event EventOpenandCloseDoor
  (params (PlayerController :type BP%20PC%20Main%20Player%20Controller%20Object%20Reference))
  (bind _garagedoor (Variables|Default|GetGarageDoor))
  (Utilities|FlowControl|DoOnce false
    (:Completed
      (Variables|Default|SetStartOpen true)
      (CallFunction|SetLightsIntensity (Variables|Default|GetInitialIntensity))
      (Utilities|FlowControl|Delay 3.0)
      (Utilities|TriggerNoisefromAudioSource (Variables|Default|GetGarageAudioSource) 0.0 (Transformation|GetWorldLocation (Variables|Default|GetGarageDoor)) self 5e+04)
      (Components|Animation|PlayAnimation _garagedoor "/Game/Props3D/Labo/PièceLabo/Garage/AS_PorteGarage.AS_PorteGarage" false)
      (Components|Timeline|SetPlayRate _garagedoor 0.2225)
      (Utilities|FlowControl|Delay 12.0)
      (CallFunction|SetLightsIntensity 0.0)
      (Variables|Default|SetStartOpen false))))

(event EventTick
  (params (DeltaSeconds :type Float%20%28single-precision%29))
  (if (Variables|Default|GetStartOpen)
    (Transformation|AddLocalRotation (Variables|Default|GetSpotLightUP) (* (Math|Rotator|MakeRotator 0.0 0.0 (Variables|Default|GetTurnSpeed)) DeltaSeconds) false false)))

(fn ConstructionScript
  (|CallParentFunction)
  (Components|DestroyComponent (Variables|Default|GetPoignees)))

(fn SetLightsIntensity
  (params (NewIntensity :type Float%20%28single-precision%29))
  (Rendering|Components|Light|SetIntensity (Variables|Default|GetSpotLightUP) NewIntensity)
  (Rendering|Components|Light|SetIntensity (Variables|Default|GetSpotLightDOWN) NewIntensity))