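; BP_Door is an interactable door that swings away from the player and lets navigating actors pass.
; Interact picks the swing sign from the player camera's facing, then a timeline rotates the mesh, reversing to close.
; When the timeline finishes, it toggles the closed state, plays a sound and reports an AI noise event.
; A child NavLinkProxy's smart link temporarily handles traversal by teleporting the moving actor to its destination.
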(event Custom|LinkReached
  (params (MovingActor :type Actor%20Object%20Reference) (DestinationPoint :type Vector%20%28by%20ref%29))
  ;[1 1 1] Temp
  (Transformation|Teleport MovingActor DestinationPoint "0, 0, 0"))

(event EventBeginPlay
  (|CallParentFunction)
  (bind _asnav_link_proxy (Utilities|Casting|CastToNavLinkProxy (Variables|/Script/Engine.ChildActorComponent|GetChildActor (Variables|Default|GetNavLink))))
  (EventDispatchers|BindEventtoOnSmartLinkReached _asnav_link_proxy (EventDispatchers|CreateEvent :!event Custom|LinkReached)))

(event EventInteract
  (params (MainPlayerController :type BP%20PC%20Main%20Player%20Controller%20Object%20Reference))
  (bind _staticmesh (Variables|Default|GetStaticMesh))
  (bind _returnvalue (Transformation|GetWorldLocation _staticmesh))
  (if (Variables|OpenDoor|GetIsClosed)
    (if (>= (Math|Vector|DotProduct (* (Math|Vector|GetForwardVector (Variables|Default|GetStaticMesh)) -1.0) (Math|Vector|GetForwardVector (Variables|/Game/Blueprints/BP_Player.BP_Player_C|GetFirstPersonCamera (Variables|/Game/Blueprints/Managers/BP_PC_MainPlayerController.BP_PC_MainPlayerController_C|GetBP_Player MainPlayerController)))) 0.0)
      (Variables|OpenDoor|SetFactor 1)
      (bind _rotationdoor (Timeline|OpenDoor Play)
        (:Update
          (Transformation|SetRelativeRotation (Variables|Default|GetStaticMesh) (Math|Rotator|MakeRotator 0.0 0.0 (* (Variables|OpenDoor|GetFactor) _rotationdoor)) false false))
        (:Finished
          (Variables|OpenDoor|SetIsClosed (not (Variables|OpenDoor|GetIsClosed)))
          ;[1 0.7048 0.02767] Missing sound
          (Audio|PlaySoundatLocation 0 _returnvalue "0, 0, 0" 1.0 1.0 0.0 0 0 0)
          (Class|AISenseHearing|ReportNoiseEvent _returnvalue 1.0 self 2.5e+03 "Noise")))
      (else
        (Variables|OpenDoor|SetFactor -1)
        (Timeline|OpenDoor Play)))
    (else
      (Timeline|OpenDoor Reverse))))

(fn ConstructionScript
  (|CallParentFunction))