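; Sliding double lab door that opens on trigger box overlap, unless a linked Generator exists and is not enabled.
; BeginPlay caches closed positions and derives open ones by offsetting each leaf along Y by its mesh bounds.
; The OpenDoors timeline lerps both leaves, reversing 2.5 seconds after an overlap ends.
; Each timeline finish triggers a noise at the door, with the stored overlapping actor as instigator.
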(event OnComponentBeginOverlap(TriggerBox)
  (params (OverlappedComponent :type Primitive%20Component%20Object%20Reference) (OtherActor :type Actor%20Object%20Reference) (OtherComp :type Primitive%20Component%20Object%20Reference) (OtherBodyIndex :type Integer) (bFromSweep :type Boolean) (SweepResult :type Hit%20Result%20Structure%20%28by%20ref%29))
  (bind _generator (Variables|Default|GetGenerator))
  (Variables|Default|SetActorInBox OtherActor)
  (if (not (Utilities|IsValid _generator))
    (bind _translation (Timeline|OpenDoors Play)
      (:Update
        (Utilities|FlowControl|Sequence
          (:then_0
            (Transformation|SetRelativeLocation (Variables|LeftDoor|GetLeftDoor) (Math|Vector|Lerp(Vector) (Variables|LeftDoor|GetCurrentLeftDoorPosition) (Variables|LeftDoor|GetNewLeftDoorPosition) _translation) false false))
          (:then_1
            (Transformation|SetRelativeLocation (Variables|RightDoor|GetRightDoor) (Math|Vector|Lerp(Vector) (Variables|RightDoor|GetCurrentRightDoorPosition) (Variables|RightDoor|GetNewRightDoorPosition) _translation) false false))))
      (:Finished
        (Utilities|TriggerNoise 0 (Transformation|GetWorldLocation (Variables|Default|GetDefaultSceneRoot)) (Variables|Default|GetActorInBox) 2.5e+03 :!pinned true) ; Missing noise
      ))
    (elif (Variables|/Game/Blueprints/Puzzles/BP_Generator.BP_Generator_C|GetIsEnable _generator)
      (Timeline|OpenDoors Play))))

(event OnComponentEndOverlap(TriggerBox)
  (params (OverlappedComponent :type Primitive%20Component%20Object%20Reference) (OtherActor :type Actor%20Object%20Reference) (OtherComp :type Primitive%20Component%20Object%20Reference) (OtherBodyIndex :type Integer))
  (Variables|Default|SetActorInBox 0)
  (Utilities|FlowControl|Delay 2.5)
  (bind _translation (Timeline|OpenDoors Reverse)
    (:Update
      (Utilities|FlowControl|Sequence
        (:then_0
          (Transformation|SetRelativeLocation (Variables|LeftDoor|GetLeftDoor) (Math|Vector|Lerp(Vector) (Variables|LeftDoor|GetCurrentLeftDoorPosition) (Variables|LeftDoor|GetNewLeftDoorPosition) _translation) false false))
        (:then_1
          (Transformation|SetRelativeLocation (Variables|RightDoor|GetRightDoor) (Math|Vector|Lerp(Vector) (Variables|RightDoor|GetCurrentRightDoorPosition) (Variables|RightDoor|GetNewRightDoorPosition) _translation) false false))))
    (:Finished
      (Utilities|TriggerNoise 0 (Transformation|GetWorldLocation (Variables|Default|GetDefaultSceneRoot)) (Variables|Default|GetActorInBox) 2.5e+03 :!pinned true) ; Missing noise
    )))

(event EventBeginPlay
  (|SetLeftDoorVariables)
  (|SetRightDoorVariables))

(fn ConstructionScript)