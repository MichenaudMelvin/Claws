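; BP_ElectricDoor is a child door Blueprint that only responds to the player while its assigned Generator is enabled.
; The IsGeneratorEnable macro gates interaction, interaction feedback and radius enter/exit events, forwarding each to the parent only when powered.
; BeginPlay reports an error and skips parent initialization if no valid Generator is assigned.
; A CheckIfDoorIsInList helper compares list entries against this door.
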(event EventBeginPlay
  (Utilities|IsValid (Variables|Default|GetGenerator)
    (:Is%20Valid
      (|CallParentFunction))
    (:Is%20Not%20Valid
      (Utilities|ErrorMessage "n'est pas affecté au générateur"))))

(event EventFeedbackCanInteract
  ;[1 1 1] Feedback interaction
  (Utilities|IsGeneratorEnable
    (:true
      (|CallParentFunction))))

(event EventFeedbackStopCanInteract
  ;[1 1 1] Feedback interaction
  (Utilities|IsGeneratorEnable
    (:true
      (|CallParentFunction))))

(event EventInteract
  (params (MainPlayerController :type BP%20PC%20Main%20Player%20Controller%20Object%20Reference))
  ;[1 1 1] Interaction
  (Utilities|IsGeneratorEnable
    (:true
      (|CallParentFunction MainPlayerController))))

(event EventEnterInteractionRadius
  (params (OtherActor :type Actor%20Object%20Reference))
  ;[1 1 1] Feedback interaction
  (Utilities|IsGeneratorEnable
    (:true
      (|CallParentFunction OtherActor))))

(event EventExitInteractionRadius
  (params (OtherActor :type Actor%20Object%20Reference))
  ;[1 1 1] Feedback interaction
  (Utilities|IsGeneratorEnable
    (:true
      (|CallParentFunction OtherActor))))

(fn ConstructionScript
  (|CallParentFunction))

(fn CheckifDoorIsinList
  (params (List :type Array%20of%20BP%20Electric%20Door%20Object%20References))
  (for (_array_element _array_index) List
    (return (== _array_element self) _array_element _array_index))
  (return false 0 0))