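; BP_TriggerEnd is an overlap trigger that shows the game's ending screen when the player reaches it.
; On BeginPlay it pre-creates a WBP_EndingScreen widget and stores it.
; The first overlap by a BP_Player, gated by a class check and DoOnce, sets the player's IsSafe flag and adds that widget to the viewport.
; An OpenLevel call to an "EndingScreen" level is left disconnected and never runs.
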(event EventBeginPlay
  (|CallParentFunction)
  (bind _returnvalue (UserInterface|CreateWidget "/Game/UI/MenuWidgets/EndingScreen/WBP_EndingScreen.WBP_EndingScreen_C"))
  (Variables|Default|SetWidgetEndingScreen _returnvalue))

(event Collision|EventActorBeginOverlap
  (params (OtherActor :type Actor%20Object%20Reference))
  (|CallParentFunction OtherActor)
  (bind _returnobject (Utilities|CheckTargetClass OtherActor "/Game/Blueprints/BP_Player.BP_Player_C")
    (:true
      (Utilities|FlowControl|DoOnce false
        (:Completed
          (bind _asbp_player (Utilities|Casting|CastToBP_Player _returnobject))
          (Variables|/Game/Blueprints/BP_Player.BP_Player_C|SetIsSafe _asbp_player true)
          (UserInterface|Viewport|AddtoViewport (Variables|Default|GetWidgetEndingScreen) 0))))))

(fn ConstructionScript
  (|CallParentFunction))