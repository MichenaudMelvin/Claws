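; Scripted-event trigger that spawns a BP_MonsterIA and walks it along a designer-set path when the player overlaps on the target entry count.
; The construction script turns PositionList into scene components, whose world locations serve as spawn point and successive AIMoveTo destinations.
; The monster is flagged as scripted during the walk; at path end the trigger destroys itself and either releases or destroys the monster.
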(event Custom|MoveToNextPosition
  (AI|AIMoveTo (Variables|Default|GetSpawnedMonster) (Transformation|GetWorldLocation (Utilities|Array|Get(acopy) (Variables|Default|GetWorldPositionList) (- (Variables|Default|GetCurrentIndex) 1))) 0 5.0 false
    (:OnSuccess
      (if (== (Variables|Default|GetCurrentIndex) (Utilities|Array|Length (Variables|Default|GetWorldPositionList)))
        (Actor|DestroyActor)
        (if (Variables|Editable|GetKeepMonsterAliveAfterPath)
          (Utilities|SetonScriptedEvent (Variables|Default|GetSpawnedMonster) false)
          (else
            (Actor|DestroyActor (Variables|Default|GetSpawnedMonster))))
        (else
          (Math|Integer|IncrementInt (Variables|Default|GetCurrentIndex)
            (:%20%20
              (CallFunction|MovetoNextPosition))))))
    (:OnFail
      (if (|CheckIfSeeThePlayer)
        (Development|PrintString (Utilities|String|Append (Utilities|GetDisplayName self) " failled, vector " (Utilities|String|ToString(Integer) (- (Variables|Default|GetCurrentIndex) 1)) " à repositionner") true true "(R=1.000000,G=0.000000,B=0.000000,A=1.000000)" 99999.0)))))

(event Collision|EventActorBeginOverlap
  (params (OtherActor :type Actor%20Object%20Reference))
  (|CallParentFunction OtherActor)
  (if (== (Variables|Default|GetEnterTriggerNumber) (Variables|Default|GetTargetEnterTime))
    (Utilities|CheckTargetClass OtherActor "/Game/Blueprints/BP_Player.BP_Player_C"
      (:true
        (bind _returnvalue (Game|SpawnActorfromClass "/Game/Blueprints/Monster/BP_MonsterIA.BP_MonsterIA_C" (Math|Conversions|ToTransform(Vector) (Transformation|GetWorldLocation (Utilities|Array|Get(acopy) (Variables|Default|GetWorldPositionList)))) "Undefined" 0 0))
        (bind _output_get (Variables|Default|SetSpawnedMonster _returnvalue))
        (Utilities|SetonScriptedEvent _output_get true)
        (CallFunction|MovetoNextPosition)))))

(fn ConstructionScript
  (|CallParentFunction)
  (for _array_element (Variables|Editable|GetPositionList)
    (bind _returnvalue (AddComponent|AddSceneComponent false (Math|Conversions|ToTransform(Vector) _array_element)))
    (Utilities|Array|Add (Variables|Default|GetWorldPositionList) _returnvalue)))