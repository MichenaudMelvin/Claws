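; Scripted event trigger that plays an assigned sound once when the player enters it.
; On overlap, it checks for BP_Player, plays PlaySound at the collision component's location, then destroys itself.
; BeginPlay reports an error if no sound is assigned.
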(event EventBeginPlay
  (Utilities|IsValid (Variables|Editable|GetPlaySound)
    (:Is%20Not%20Valid
      (Utilities|ErrorMessage "ne possede pas de son"))))

(event Collision|EventActorBeginOverlap
  (params (OtherActor :type Actor%20Object%20Reference))
  (|CallParentFunction OtherActor)
  (Utilities|CheckTargetClass OtherActor "/Game/Blueprints/BP_Player.BP_Player_C"
    (:true
      (Audio|PlaySoundatLocation (Variables|Editable|GetPlaySound) (Transformation|GetWorldLocation (Variables|Default|GetCollisionComponent)) "0, 0, 0" 1.0 1.0 0.0 0 0 0)
      (Actor|DestroyActor))))

(fn ConstructionScript
  (|CallParentFunction))