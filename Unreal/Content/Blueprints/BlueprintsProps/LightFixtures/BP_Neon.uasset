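; Neon light fixture prop with a rect light that follows the generator state in the save data.
; Shortly after BeginPlay it lights up if the generator is enabled, otherwise hides the light; ToggleLightVisibility also switches it.
; Toggling, gated by DoLight, applies the emissive LED material even when switching off, sets a hardcoded intensity and starts optional blinking.
; The construction script previews the light through an editor visibility flag.
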(event EventBeginPlay
  (bind _mainsaveddata (CallFunction|GetMainSaveData))
  (bind _isgeneratorenable (Variables|/Game/Blueprints/Checkpoints/BP_SavedData.BP_SavedData_C|GetIsGeneratorEnable _mainsaveddata))
  (|CallParentFunction)
  (Utilities|FlowControl|Delay 0.2)
  (Utilities|IsValid _mainsaveddata
    (:Is%20Valid
      (if _isgeneratorenable
        (CallFunction|ToggleVisibility _isgeneratorenable)
        (else
          (Rendering|SetVisibility (Variables|Default|GetRectLight) false false :!label _label))))
    (:Is%20Not%20Valid
      (goto _label))))

(event EventToggleLightVisibility
  (params (Visibility :type Boolean))
  (CallFunction|ToggleVisibility Visibility))

(fn ConstructionScript
  (bind _editorvisibilty (Variables|Editable|GetEditorVisibilty))
  (bind _rectlight (Variables|Default|GetRectLight))
  (|CallParentFunction)
  (Rendering|SetVisibility _rectlight _editorvisibilty false)
  (Rendering|Components|Light|SetIntensity _rectlight (Math|Float|SelectFloat 1.6e+02 0.0 _editorvisibilty)))

(fn ToggleVisibility
  (params (Visibility :type Boolean))
  (bind _rectlight (Variables|Default|GetRectLight))
  (if (Variables|Editable|GetDoLight)
    (Rendering|Material|SetMaterial (Variables|Default|GetModularMesh) 1 "/Game/Materials/Labo/LED/M_LED_LightEmisive.M_LED_LightEmisive")
    (Rendering|SetVisibility _rectlight Visibility true)
    (Rendering|Components|Light|SetIntensity _rectlight 1.6e+02) ; dégeu, jdevrai le faire avec une variable mais pas trop le temps
    (if (and Visibility (Variables|Default|GetCanBlink))
      (CallFunction|Blink (Variables|Default|GetRectLight)))))