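; Abstract base Blueprint for light fixture props, providing a random flicker effect and a visibility hook.
; The Blink event randomly either cuts a given light's intensity to zero briefly and restores it, or waits a random interval.
; It re-calls itself to loop for as long as that light is visible.
; ToggleVisibility is an empty function, and the construction script only calls the parent.
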(event Custom|Blink
  (params (Light :type Light%20Component%20Object%20Reference))
  (if (Rendering|IsVisible Light)
    (if (Math|Random|RandomBool)
      (Variables|Default|SetTempIntensity (Variables|/Script/Engine.LightComponentBase|GetIntensity Light))
      (Rendering|Components|Light|SetIntensity Light 0.0)
      (Utilities|FlowControl|Delay 0.1)
      (Rendering|Components|Light|SetIntensity Light (Variables|Default|GetTempIntensity))
      (else
        (Utilities|FlowControl|Delay (Math|Random|RandomFloatinRange 0.5 1e+01))))
    (CallFunction|Blink Light)))

(fn ConstructionScript
  (|CallParentFunction))

(fn ToggleVisibility
  (params (Visibility :type Boolean)))