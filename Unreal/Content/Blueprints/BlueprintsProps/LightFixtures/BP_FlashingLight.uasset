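; Flashing light fixture prop that spins two spotlights, SpotLightUP and SpotLightDOWN, to act as a rotating beacon.
; On BeginPlay it passes both spotlights to UpdateIntensity, which is not defined in this graph.
; Each Tick adds local yaw to both lights at TurnSpeed scaled by delta time, so the motion is frame-rate independent.
; The construction script only runs the parent's.
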(event EventBeginPlay
  (CallFunction|UpdateIntensity (Utilities|Array|MakeArray (Variables|Default|GetSpotLightUP) (Variables|Default|GetSpotLightDOWN))))

(event EventTick
  (params (DeltaSeconds :type Float%20%28single-precision%29))
  (Transformation|AddLocalRotation (Variables|Default|GetSpotLightUP) (* (Math|Rotator|MakeRotator 0.0 0.0 (Variables|Default|GetTurnSpeed)) DeltaSeconds) false false))

(fn ConstructionScript
  (|CallParentFunction))