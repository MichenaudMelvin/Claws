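; BP_LED is a light fixture prop with red and green LEDs that indicate whether the generator is enabled.
; Shortly after BeginPlay it reads IsGeneratorEnable from the main save data and shows green if on, red if off or no save is found.
; The construction script sets each LED from its visibility variable, and ToggleVisibility swaps the two before calling the parent implementation.
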(event EventBeginPlay
  (bind _mainsaveddata (CallFunction|GetMainSaveData))
  (Utilities|FlowControl|Delay 0.2)
  (Utilities|IsValid _mainsaveddata
    (:Is%20Valid
      (if (Variables|/Game/Blueprints/Checkpoints/BP_SavedData.BP_SavedData_C|GetIsGeneratorEnable _mainsaveddata)
        (Rendering|SetVisibility (Variables|Default|GetRedLED) false true)
        (Rendering|SetVisibility (Variables|Default|GetGreenLED) true true)
        (else
          (Rendering|SetVisibility (Variables|Default|GetRedLED) true true :!label _label)
          (Rendering|SetVisibility (Variables|Default|GetGreenLED) false true))))
    (:Is%20Not%20Valid
      (goto _label))))

(fn ConstructionScript
  (|CallParentFunction)
  (Rendering|SetVisibility (Variables|Default|GetRedLED) (Variables|Editable|GetRedLEDVisibility) true)
  (Rendering|SetVisibility (Variables|Default|GetGreenLED) (Variables|Editable|GetGreenLEDVisibility) true))

(fn ToggleVisibility
  (params (Visibility :type Boolean))
  (Rendering|SetVisibility (Variables|Default|GetRedLED) (not Visibility) false)
  (Rendering|SetVisibility (Variables|Default|GetGreenLED) Visibility false)
  (|CallParentFunction Visibility))