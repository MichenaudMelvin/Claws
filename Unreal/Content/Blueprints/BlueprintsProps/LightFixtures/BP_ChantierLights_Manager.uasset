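; Manager for the construction-site lights that switches on every BP_SpotChantier in the level when the OverallGeneratorFuseSnapped event fires.
; It gathers the spots with GetAllActorsOfClass and steps through them with a delayed loop, so they light up in a staggered sequence with a debug print for each.
; A Sort function meant to order elements by their Index is never run, so the sequence follows the unsorted query order.
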(event EventOverallGeneratorFuseSnapped
  (bind _outactors (Actor|GetAllActorsOfClass "/Game/Blueprints/BlueprintsProps/LightFixtures/BP_SpotChantier.BP_SpotChantier_C"))
  (bind _arrayelement (Utilities|ForEachLoopDelay _outactors 0.5)
    (:LoopBody
      (Class|BIGameEventsManager|ChantiersLightTurnon(Message) _arrayelement)
      (Development|PrintString (Utilities|String|Append "LIGHT TURN ON: " (Utilities|GetDisplayName _arrayelement))))))

(fn ConstructionScript)

(fn Sort
  (params (NewParam :type Array%20of%20BP%20Spot%20Chantier%20Object%20References))
  (for _array_element NewParam
    (Utilities|Array|Insert (LocalVariables|GetArrayReturn) _array_element (Variables|/Game/Blueprints/BlueprintsProps/LightFixtures/BP_SpotChantier.BP_SpotChantier_C|GetIndex _array_element)))
  (return (LocalVariables|GetArrayReturn)))