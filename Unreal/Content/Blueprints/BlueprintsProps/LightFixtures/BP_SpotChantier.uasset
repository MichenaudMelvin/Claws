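; Construction-site ("chantier") spotlight fixture whose two spot lights start dark unless the saved generator state is enabled.
; BeginPlay reads the save after a short delay; the generator-on branch calls the deprecated, empty ToggleLightVisibility.
; ChantiersLightTurnon shows both lights and fades their intensity up with a timeline.
; The construction script previews lighting through EditorVisibilty and parses Index from the object name's "Chantier_" suffix.
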(event EventBeginPlay
  (bind _mainsaveddata (CallFunction|GetMainSaveData))
  (bind _isgeneratorenable (Variables|/Game/Blueprints/Checkpoints/BP_SavedData.BP_SavedData_C|GetIsGeneratorEnable _mainsaveddata))
  (|CallParentFunction)
  (Utilities|FlowControl|Delay 0.2)
  (Utilities|IsValid _mainsaveddata
    (:Is%20Valid
      (if _isgeneratorenable
        (CallFunction|ToggleLightVisibility _isgeneratorenable)
        (else
          (Rendering|SetVisibility (Variables|Default|GetSpotLight1) false false :!label _label)
          (Rendering|Components|Light|SetIntensity (Variables|Default|GetSpotLight1) 0.0)
          (Rendering|Components|Light|SetIntensity (Variables|Default|GetSpotLight) 0.0))))
    (:Is%20Not%20Valid
      (goto _label))))

(event EventToggleLightVisibility
  (params (Visibility :type Boolean))
  ;[1 1 1] Deprecated by BI_GameEvents_Manager (gameplay event message)
)

(event EventChantiersLightTurnon
  (Rendering|SetVisibility (Variables|Default|GetSpotLight1) true false)
  (Rendering|SetVisibility (Variables|Default|GetSpotLight) true false)
  (bind _alpha_value (Timeline|ChantierLight_TurnOn_Fader Play)
    (:Update
      (Rendering|Components|Light|SetIntensity (Variables|Default|GetSpotLight1) (Math|Float|Lerp 0.0 2e+03 _alpha_value))
      (Rendering|Components|Light|SetIntensity (Variables|Default|GetSpotLight) (Math|Float|Lerp 0.0 2e+03 _alpha_value)))))

(fn ConstructionScript
  (bind _editor_visibilty (Variables|Default|GetEditor%20Visibilty))
  (bind _returnvalue (Math|Float|SelectFloat 2e+03 0.0 _editor_visibilty))
  (|CallParentFunction)
  (Rendering|SetVisibility (Variables|Default|GetSpotLight1) _editor_visibilty false)
  (Rendering|Components|Light|SetIntensity (Variables|Default|GetSpotLight1) _returnvalue)
  (Rendering|Components|Light|SetIntensity (Variables|Default|GetSpotLight) _returnvalue)
  (Variables|Default|SetIndex (Math|Conversions|ToInteger(Byte) (.RightS (Utilities|String|Split (Utilities|GetObjectName self) "Chantier_")))))