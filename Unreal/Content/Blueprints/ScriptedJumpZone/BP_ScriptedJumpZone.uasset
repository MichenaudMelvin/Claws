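; BP_ScriptedJumpZone is an interactable zone that teleports the player to a scripted destination.
; On Interact, it takes the player from the passed MainPlayerController and calls Teleport to the static mesh's world location plus the EmplacementToGo offset, with zero rotation.
; The move is instantaneous, with no jump motion, and the overlap event is empty.
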(event EventBeginPlay
  (|CallParentFunction) ; This node is disabled and will not be called.\nDrag off pins to build functionality.
)

(event Collision|EventActorBeginOverlap
  (params (OtherActor :type Actor%20Object%20Reference)))

(event EventTick
  (params (DeltaSeconds :type Float%20%28single-precision%29))
  (|CallParentFunction DeltaSeconds) ; This node is disabled and will not be called.\nDrag off pins to build functionality.
)

(event EventInteract
  (params (MainPlayerController :type BP%20PC%20Main%20Player%20Controller%20Object%20Reference))
  (Transformation|Teleport (Variables|/Game/Blueprints/Managers/BP_PC_MainPlayerController.BP_PC_MainPlayerController_C|GetBP_Player MainPlayerController) (+ (Variables|Default|GetEmplacementToGo) (Transformation|GetWorldLocation (Variables|Default|GetStaticMesh))) "0, 0, 0"))

(fn ConstructionScript
  (|CallParentFunction))