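; BP_MonsterIA is the AI-controlled monster that damages the player and reacts to being hit by a vial (BP_Fiole).
; Vial overlaps set the ReceiveFiole flag, destroy the vial and show a one-time tip.
; AttackCollision starts disabled and damages players unless safe, while RealCollision hits ignore safety; each damages only once, never during the death screen.
; GetBlackBoard exposes the monster controller's blackboard.
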(event OnComponentBeginOverlap(FioleCollider)
  (params (OverlappedComponent :type Primitive%20Component%20Object%20Reference) (OtherActor :type Actor%20Object%20Reference) (OtherComp :type Primitive%20Component%20Object%20Reference) (OtherBodyIndex :type Integer) (bFromSweep :type Boolean) (SweepResult :type Hit%20Result%20Structure%20%28by%20ref%29))
  (bind _returnobject (Utilities|CheckTargetClass OtherActor "/Game/Blueprints/Fioles/BP_Fiole.BP_Fiole_C")
    (:true
      (bind _asbp_fiole (Utilities|Casting|CastToBP_Fiole _returnobject))
      (Utilities|SetBoolValue "ReceiveFiole" true)
      (Default|DestroyObject _asbp_fiole)
      (Utilities|FlowControl|DoOnce false
        (:Completed
          (Default|ShowSingleTip (Variables|/Game/Blueprints/Managers/BP_PC_MainPlayerController.BP_PC_MainPlayerController_C|GetTipWidget (CallFunction|CallMainPlayerController)) (Utilities|Struct|MakeSTRUCT_Tip "Take that, you little shit !" 5.0)))))))

(event OnComponentBeginOverlap(AttackCollision)
  (params (OverlappedComponent :type Primitive%20Component%20Object%20Reference) (OtherActor :type Actor%20Object%20Reference) (OtherComp :type Primitive%20Component%20Object%20Reference) (OtherBodyIndex :type Integer) (bFromSweep :type Boolean) (SweepResult :type Hit%20Result%20Structure%20%28by%20ref%29))
  (bind _returnobject (Utilities|CheckTargetClass OtherActor "/Game/Blueprints/BP_Player.BP_Player_C")
    (:true
      (bind _asbp_player (Utilities|Casting|CastToBP_Player _returnobject))
      (if (and (not (Variables|/Game/Blueprints/BP_Player.BP_Player_C|GetIsSafe _asbp_player)) (not (UserInterface|Viewport|IsinViewport (Variables|/Game/Blueprints/Managers/BP_PC_MainPlayerController.BP_PC_MainPlayerController_C|GetDeathScreenWidget (Variables|/Game/Blueprints/BP_Player.BP_Player_C|GetPlayerController _asbp_player)))))
        (Utilities|FlowControl|DoOnce false
          (:Completed
            (Default|TakeDamages (Variables|/Game/Blueprints/BP_Player.BP_Player_C|GetPlayerController _asbp_player))))))))

(event OnComponentHit(RealCollision)
  (params (HitComponent :type Primitive%20Component%20Object%20Reference) (OtherActor :type Actor%20Object%20Reference) (OtherComp :type Primitive%20Component%20Object%20Reference) (NormalImpulse :type Vector :default "0, 0, 0") (Hit :type Hit%20Result%20Structure%20%28by%20ref%29))
  (bind _returnobject (Utilities|CheckTargetClass OtherActor "/Game/Blueprints/BP_Player.BP_Player_C")
    (:true
      (bind _asbp_player (Utilities|Casting|CastToBP_Player _returnobject))
      (if (not (UserInterface|Viewport|IsinViewport (Variables|/Game/Blueprints/Managers/BP_PC_MainPlayerController.BP_PC_MainPlayerController_C|GetDeathScreenWidget (Variables|/Game/Blueprints/BP_Player.BP_Player_C|GetPlayerController _asbp_player))))
        (Utilities|FlowControl|DoOnce false
          (:Completed
            (Default|TakeDamages (Variables|/Game/Blueprints/BP_Player.BP_Player_C|GetPlayerController _asbp_player))))))))

(event EventBeginPlay
  (bind _asaicontroller (Utilities|Casting|CastToAIController (Pawn|GetController)))
  (Variables|Default|SetAIController _asaicontroller)
  (Collision|SetCollisionEnabled (Variables|Default|GetAttackCollision) "NoCollision"))

(fn ConstructionScript)

(fn GetBlackBoard
  (bind _asbp_aic_monster_controller (Utilities|Casting|CastToBP_AIC_MonsterController (AI|GetAIController self)))
  (return (Variables|/Game/Blueprints/Monster/BP_AIC_MonsterController.BP_AIC_MonsterController_C|GetBlackboard%20Ref _asbp_aic_monster_controller)))