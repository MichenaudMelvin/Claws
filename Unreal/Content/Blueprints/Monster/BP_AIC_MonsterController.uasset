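; AI controller for the monster that starts its blackboard and behavior tree and translates perception events into blackboard state.
; Noise stimuli set the sound location and flags that distinguish a first heard sound from a new one arriving while already searching or alerted.
; Non-noise stimuli from the player, treated as vision, update whether the player has been seen and clear the scripted-behavior flag.
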(event OnPerceptionUpdated(AIPerception)
  (params (UpdatedActors :type Array%20of%20Actor%20Object%20References))
  (for _array_element UpdatedActors
    (bind _info (Class|AIPerceptionComponent|GetActorsPerception (Variables|AI|GetAIPerception) _array_element))
    (for _array_element_2 (.LastSensedStimuli (Utilities|Struct|BreakActorPerceptionBlueprintInfo _info))
      (if (Utilities|Name|Equal(Name) (.Tag (Utilities|Struct|BreakAIStimulus _array_element_2)) "Noise")
        (if (or (Utilities|GetBoolValue "HeardOneSound") (Utilities|GetBoolValue "SearchingSound"))
          (Utilities|SetBoolValue "StartMoveTo" false)
          (Utilities|SetBoolValue "HearNewSound" (.bSuccessfullySensed (Utilities|Struct|BreakAIStimulus _array_element_2)))
          (Utilities|SetBoolValue "SearchingSound" false)
          (else
            (Utilities|SetBoolValue "SearchingSound" (.bSuccessfullySensed (Utilities|Struct|BreakAIStimulus _array_element_2)))
            (Utilities|SetBoolValue "HeardOneSound" true)))
        (Utilities|SetVectorValue "SoundLocation" (.StimulusLocation (Utilities|Struct|BreakAIStimulus _array_element_2)))))))

(event OnTargetPerceptionUpdated(AIPerception)
  (params (Actor :type Actor%20Object%20Reference) (Stimulus :type AI%20Stimulus%20Structure))
  (bind (_age _expirationage _strength _stimuluslocation _receiverlocation _tag _bsuccessfullysensed) (Utilities|Struct|BreakAIStimulus Stimulus))
  (Utilities|CheckTargetClass Actor "/Game/Blueprints/BP_Player.BP_Player_C"
    (:true
      (if (Utilities|Name|NotEqual(Name) _tag "Noise")
        (Utilities|SetBoolValue "HasSeenPlayer" _bsuccessfullysensed)
        (Utilities|SetBoolValue "IsScripted" false)))))

(event EventBeginPlay
  (bind _blackboardcomponent (Class|AIController|UseBlackboard "/Game/Blueprints/Monster/BB_Monster.BB_Monster"))
  (Variables|Default|SetBlackboard%20Ref _blackboardcomponent)
  (AI|RunBehaviorTree "/Game/Blueprints/Monster/BT_Monster.BT_Monster"))

(fn ConstructionScript)