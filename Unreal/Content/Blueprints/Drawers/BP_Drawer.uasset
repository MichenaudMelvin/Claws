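; BP_Drawer is an interactable drawer that slides open and closed, alternating on each interaction.
; BeginPlay sets the open position 50 units along the mesh's forward vector from the actor location.
; Interact flips between playing and reversing a timeline that lerps the mesh's world location between both positions.
; Each interaction also reports a "Noise" event instigated by the player, while its sound call has no asset assigned.
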(event EventBeginPlay
  (|CallParentFunction)
  (bind _output_get (Variables|Positions|SetCurrentPosition (Transformation|GetActorLocation)))
  (Variables|Positions|SetDestination (+ _output_get (* (Math|Vector|GetForwardVector (Variables|Default|GetStaticMesh)) 50))))

(event EventInteract
  (params (MainPlayerController :type BP%20PC%20Main%20Player%20Controller%20Object%20Reference))
  (bind _staticmesh (Variables|Default|GetStaticMesh))
  (bind _returnvalue (Transformation|GetWorldLocation _staticmesh))
  ;[1 0.8132 0.03339] Missing sound
  (Audio|PlaySoundatLocation 0 _returnvalue "0, 0, 0" 1.0 1.0 0.0 0 0 0)
  (Class|AISenseHearing|ReportNoiseEvent _returnvalue 1.0 (Variables|/Game/Blueprints/Managers/BP_PC_MainPlayerController.BP_PC_MainPlayerController_C|GetBP_Player MainPlayerController) 1e+03 "Noise")
  (Utilities|FlowControl|FlipFlop
    (:A
      (bind _translationvalue (Timeline|Translation Play)
        (:Update
          (Transformation|SetWorldLocation (Variables|Default|GetStaticMesh) (Math|Vector|Lerp(Vector) (Variables|Positions|GetCurrentPosition) (Variables|Positions|GetDestination) _translationvalue) false false))))
    (:B
      (Timeline|Translation Reverse))))

(fn ConstructionScript
  (|CallParentFunction))