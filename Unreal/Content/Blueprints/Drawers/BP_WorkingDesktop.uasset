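; BP_WorkingDesktop is a desk Blueprint that registers eight child actor components as its drawers.
; Its construction script appends each component to DrawerList, then calls the parent construction script, so the list is filled before the parent logic runs.
; The event graph holds only disabled placeholder events, so any runtime drawer behavior lies outside this graph.
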(event EventBeginPlay)

(event Collision|EventActorBeginOverlap
  (params (OtherActor :type Actor%20Object%20Reference)))

(event EventTick
  (params (DeltaSeconds :type Float%20%28single-precision%29)))

(fn ConstructionScript
  (for _array_element (Utilities|Array|MakeArray (Variables|Default|GetChildActor1) (Variables|Default|GetChildActor2) (Variables|Default|GetChildActor3) (Variables|Default|GetChildActor4) (Variables|Default|GetChildActor5) (Variables|Default|GetChildActor6) (Variables|Default|GetChildActor7) (Variables|Default|GetChildActor8))
    (Utilities|Array|Add (Variables|Default|GetDrawerList) _array_element))
  (|CallParentFunction))