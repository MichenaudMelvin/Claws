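; BP_Drawers is an interactable drawer that slides open and closed when a player uses it.
; Its data supplies the mesh at construction and the slide distance along the mesh's forward vector, computed at BeginPlay.
; Each interaction triggers a noise at the mesh, attributed to the player, then a FlipFlop plays or reverses a timeline that lerps the mesh between start and destination.
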(event EventBeginPlay
  (|CallParentFunction)
  (bind _output_get (Variables|Positions|SetCurrentPosition (Transformation|GetActorLocation)))
  (Variables|Positions|SetDestination (+ _output_get (* (Math|Vector|GetForwardVector (Variables|Default|GetStaticMesh)) (Variables|/Game/Blueprints/Drawers/BP_DA_Drawer.BP_DA_Drawer_C|GetTranslationValue (Variables|Data|GetData))))))

(event EventInteract
  (params (MainPlayerController :type BP%20PC%20Main%20Player%20Controller%20Object%20Reference))
  (Utilities|TriggerNoise 0 (Transformation|GetWorldLocation (Variables|Default|GetStaticMesh)) (Variables|/Game/Blueprints/Managers/BP_PC_MainPlayerController.BP_PC_MainPlayerController_C|GetBP_Player MainPlayerController) 1e+03) ; Missing noise
  (Utilities|FlowControl|FlipFlop
    (:A
      (bind _translationvalue (Timeline|Translation Play)
        (:Update
          (Transformation|SetWorldLocation (Variables|Default|GetStaticMesh) (Math|Vector|Lerp(Vector) (Variables|Positions|GetCurrentPosition) (Variables|Positions|GetDestination) _translationvalue) false false))))
    (:B
      (Timeline|Translation Reverse))))

(fn ConstructionScript
  (|CallParentFunction)
  (Components|StaticMesh|SetStaticMesh (Variables|Default|GetStaticMesh) (Variables|/Game/Blueprints/Drawers/BP_DA_Drawer.BP_DA_Drawer_C|GetMesh (Variables|Data|GetData))))