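; BP_Desktop is a desk with drawers that also acts as a safe spot for the player.
; Its construction script fills DrawerList with three child actor components, then runs the parent construction script.
; Overlap events on the SafeZone component check for BP_Player and set its IsSafe flag on entry, clearing it on exit.
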(event OnComponentBeginOverlap(SafeZone)
  (params (OverlappedComponent :type Primitive%20Component%20Object%20Reference) (OtherActor :type Actor%20Object%20Reference) (OtherComp :type Primitive%20Component%20Object%20Reference) (OtherBodyIndex :type Integer) (bFromSweep :type Boolean) (SweepResult :type Hit%20Result%20Structure%20%28by%20ref%29))
  (bind _returnobject (Utilities|CheckTargetClass OtherActor "/Game/Blueprints/BP_Player.BP_Player_C")
    (:true
      (bind _asbp_player (Utilities|Casting|CastToBP_Player _returnobject))
      (Variables|/Game/Blueprints/BP_Player.BP_Player_C|SetIsSafe _asbp_player true))))

(event OnComponentEndOverlap(SafeZone)
  (params (OverlappedComponent :type Primitive%20Component%20Object%20Reference) (OtherActor :type Actor%20Object%20Reference) (OtherComp :type Primitive%20Component%20Object%20Reference) (OtherBodyIndex :type Integer))
  (bind _returnobject (Utilities|CheckTargetClass OtherActor "/Game/Blueprints/BP_Player.BP_Player_C")
    (:true
      (bind _asbp_player (Utilities|Casting|CastToBP_Player _returnobject))
      (Variables|/Game/Blueprints/BP_Player.BP_Player_C|SetIsSafe _asbp_player false))))

(fn ConstructionScript
  (Variables|Default|SetDrawerList (Utilities|Array|MakeArray (Variables|Default|GetChildActor1) (Variables|Default|GetChildActor2) (Variables|Default|GetChildActor3)))
  (|CallParentFunction))