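; BP_SpecialNotes is an interactable note that shows its texture in the player controller's SpecialNoteWidget.
; Interact toggles the widget: opening passes in the note Data, stops the player's movement sound, unbinds all controls and calls BindEvents.
; BindEvents rebinds interact and hooks the notebook, pause and shoot events, while closing fades the widget out and restores basic bindings.
; Its construction script only prints a silent string to override the parent's.
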(event EventInteract
  (params (MainPlayerController :type BP%20PC%20Main%20Player%20Controller%20Object%20Reference))
  (bind _specialnotewidget (Variables|/Game/Blueprints/Managers/BP_PC_MainPlayerController.BP_PC_MainPlayerController_C|GetSpecialNoteWidget MainPlayerController))
  (bind _data (Variables|Default|GetData))
  (if (UserInterface|Viewport|IsinViewport _specialnotewidget)
    (Default|FadeOut _specialnotewidget)
    (Default|BasicBind MainPlayerController)
    (else
      (UserInterface|Viewport|AddtoViewport _specialnotewidget 0)
      (Variables|/Game/Blueprints/Notes/WBP_SpecialNote.WBP_SpecialNote_C|SetCurrentData _specialnotewidget _data)
      (Default|SetNoteText _specialnotewidget (Variables|/Game/Blueprints/Notes/BP_DA_Notes.BP_DA_Notes_C|GetTextureForSpecialNotes _data))
      (Audio|Components|Audio|Stop (Variables|/Game/Blueprints/BP_Player.BP_Player_C|GetMovementSoundSource (Variables|/Game/Blueprints/Managers/BP_PC_MainPlayerController.BP_PC_MainPlayerController_C|GetBP_Player MainPlayerController)))
      (Default|UnbindAll MainPlayerController)
      (|BindEvents MainPlayerController))))

(event EventBeginPlay
  (|CallParentFunction))

(fn ConstructionScript
  (Development|PrintString "Only for overide parent construction script" false false))