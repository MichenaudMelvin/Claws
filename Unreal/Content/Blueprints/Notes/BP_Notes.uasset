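; BP_Notes is an interactable note pickup whose mesh and blink materials come from its Data asset in the construction script.
; On BeginPlay it destroys itself if that data is already in the saved notes inventory, otherwise it marks the note unread.
; Interacting adds the data to the player controller's sorted inventory and save data, may show a tutorial tip when the inventory is empty, then destroys the actor.
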(event EventBeginPlay
  (bind _mainsaveddata (CallFunction|GetMainSaveData))
  (|CallParentFunction)
  (Utilities|IsValid (Variables|Editable|GetData)
    (:Is%20Valid
      (Utilities|IsValid _mainsaveddata
        (:Is%20Valid
          (if (CallFunction|CheckMatchingData (Variables|/Game/Blueprints/Checkpoints/BP_SavedData.BP_SavedData_C|GetPlayerNotesInventory _mainsaveddata))
            (Actor|DestroyActor)
            (else
              (Default|SetIsRead (Variables|Editable|GetData) false :!label _label))))
        (:Is%20Not%20Valid
          (goto _label))))
    (:Is%20Not%20Valid
      (Development|PrintString (Utilities|String|Append (Utilities|GetDisplayName self) " ne possède pas de data") true true "(R=1.000000,G=0.000000,B=0.000000,A=1.000000)" 99999.0))))

(event EventInteract
  (params (MainPlayerController :type BP%20PC%20Main%20Player%20Controller%20Object%20Reference))
  (bind _notesinventory (Variables|/Game/Blueprints/Managers/BP_PC_MainPlayerController.BP_PC_MainPlayerController_C|GetNotesInventory MainPlayerController))
  (if (and (Utilities|IsArrayNullPure _notesinventory) (Default|GetHasSeenNotesTutorial MainPlayerController))
    (Default|ShowSingleTip (Variables|/Game/Blueprints/Managers/BP_PC_MainPlayerController.BP_PC_MainPlayerController_C|GetTipWidget MainPlayerController) (Utilities|Struct|MakeSTRUCT_Tip (Utilities|Text|ToText(String) (Utilities|String|Append "What's that ? A note ?" "(Press " (Utilities|String|ToString(Text) (CallFunction|GetKeyActionName "InteractWithNoteBook" 1)) " to open notes inventory)")) 2.5)) ; Juste un ptit warn quand le tuto du debut est actif
    (Default|SetHasSeenNotesTurorial MainPlayerController true))
  (Utilities|Array|Add _notesinventory (Variables|Editable|GetData))
  (CallFunction|SetNoteInventoryonSave (Variables|/Game/Blueprints/Managers/BP_PC_MainPlayerController.BP_PC_MainPlayerController_C|GetNotesInventory MainPlayerController))
  (Default|SortInventory MainPlayerController)
  (Actor|DestroyActor))

(fn ConstructionScript
  (bind _data (Variables|Editable|GetData))
  (Components|StaticMesh|SetStaticMesh (Variables|Default|GetStaticMesh) (Variables|/Game/Blueprints/Notes/BP_DA_Notes.BP_DA_Notes_C|GetMesh _data))
  (CallFunction|SetStaticMaterialList (Variables|/Game/Blueprints/Notes/BP_DA_Notes.BP_DA_Notes_C|GetBlinkMaterialsList _data) (Variables|Default|GetBlinkMaterialList))
  (|CallParentFunction))

(fn CheckMatchingData
  (params (DataList :type Array%20of%20BP%20DA%20Notes%20Object%20References))
  (for _array_element DataList
    (if (== _array_element (Variables|Editable|GetData))
      (return true)))
  (return false))

(fn SetNoteInventoryonSave
  (params (PlayerNotesInventory :type Array%20of%20BP%20DA%20Notes%20Object%20References))
  (Variables|/Game/Blueprints/Checkpoints/BP_SavedData.BP_SavedData_C|SetPlayerNotesInventory (CallFunction|CallCurrentSaveData) PlayerNotesInventory))