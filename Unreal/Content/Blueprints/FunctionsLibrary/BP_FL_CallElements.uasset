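; Blueprint function library of global accessors for core game objects.
; It returns the first player's BP_PC_MainPlayerController, the player reference stored on that controller, and the current save data held by FirstPersonGameMode.
; Each lookup rests on a cast of the player controller or game mode, and the player getter reuses the controller getter.
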(fn CallMainPlayerController
  (bind _asbp_pc_main_player_controller (Utilities|Casting|CastToBP_PC_MainPlayerController (Game|GetPlayerController 0)))
  (return _asbp_pc_main_player_controller))

(fn CallPlayer
  (return (Variables|/Game/Blueprints/Managers/BP_PC_MainPlayerController.BP_PC_MainPlayerController_C|GetBP_Player (CallFunction|CallMainPlayerController))))

(fn CallCurrentSaveData
  (bind _asfirst_person_game_mode (Utilities|Casting|CastToFirstPersonGameMode (Game|GetGameMode)))
  (return (Variables|/Game/FirstPersonBP/Blueprints/FirstPersonGameMode.FirstPersonGameMode_C|GetMySaveData _asfirst_person_game_mode)))