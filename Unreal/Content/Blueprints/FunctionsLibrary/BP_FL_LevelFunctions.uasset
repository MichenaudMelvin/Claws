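; Level helper function library with a RestartLevel function that reloads the current level and aims to return the player to the last checkpoint.
; It records the current checkpoint's location if one is valid, then reopens the level by name.
; Immediately after the open call, it hides the mouse cursor, assigns SaveNotesInventory to the player controller's notes inventory, and moves the player to the recorded location.
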(fn RestartLevel
  (bind _mainplayercontroller (CallFunction|CallMainPlayerController))
  (bind _currentcheckpoint (Variables|/Game/Blueprints/Managers/BP_PC_MainPlayerController.BP_PC_MainPlayerController_C|GetCurrentCheckpoint _mainplayercontroller))
  (Utilities|IsValid _currentcheckpoint
    (:Is%20Valid
      (LocalVariables|SetLastCheckpointLocation (Transformation|GetActorLocation _currentcheckpoint)))
    (:Is%20Not%20Valid
      _))
  (bind _returnvalue (Game|GetCurrentLevelName 0))
  (Game|OpenLevel(byName) 0 (Utilities|String|StringToName _returnvalue))
  (Variables|/Script/Engine.PlayerController|SetbShowMouseCursor _mainplayercontroller false)
  (Variables|/Game/Blueprints/Managers/BP_PC_MainPlayerController.BP_PC_MainPlayerController_C|SetNotesInventory _mainplayercontroller (LocalVariables|GetSaveNotesInventory))
  (Transformation|SetActorLocation (Variables|/Game/Blueprints/Managers/BP_PC_MainPlayerController.BP_PC_MainPlayerController_C|GetBP_Player _mainplayercontroller) (LocalVariables|GetLastCheckpointLocation) false false))