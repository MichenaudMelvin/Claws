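; Blueprint function library of small input and settings helpers.
; Two getters look up an action or axis mapping in Input Settings by name and array index and return the key's display name.
; WriteMessageWithKeyAction wraps an action's key name between two strings, returning it as both string and text.
; EnableVSync sets the VSync flag on Game User Settings, without applying or saving the settings.
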(fn GetKeyActionName
  (params (ActionName :type Name) (KeyInArray :type Integer))
  (return (Class|KismetInputLibrary|KeyGetDisplayName (.Key (Utilities|Struct|BreakInputActionKeyMapping (Utilities|Array|Get(acopy) (Class|InputSettings|GetActionMappingbyName (Class|InputSettings|GetInputSettings) ActionName) KeyInArray))))))

(fn GetKeyAxisName
  (params (ActionName :type Name) (KeyInArray :type Integer))
  (return (Class|KismetInputLibrary|KeyGetDisplayName (.Key (Utilities|Struct|BreakInputAxisKeyMapping (Utilities|Array|Get(acopy) (Class|InputSettings|GetAxisMappingbyName (Class|InputSettings|GetInputSettings) ActionName) KeyInArray))))))

(fn WriteMessagewithKeyAction
  (params (A :type String) (C :type String) (ActionName :type Name) (KeyInArray :type Integer))
  (bind _keyname (CallFunction|GetKeyActionName ActionName KeyInArray))
  (bind _returnvalue (Utilities|String|ToString(Text) _keyname))
  (bind _returnvalue_2 (Utilities|String|Append A _returnvalue C))
  (return _returnvalue_2 (Utilities|Text|ToText(String) _returnvalue_2)))

(fn EnableVSync
  (params (bEnable :type Boolean))
  (bind _returnvalue (Settings|GetGameUserSettings))
  (Class|GameUserSettings|SetVSyncEnabled _returnvalue bEnable))