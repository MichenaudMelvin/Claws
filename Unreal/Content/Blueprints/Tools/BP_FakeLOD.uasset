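; BP_FakeLOD is a trigger actor that sets the in-game visibility of actors on listed layers when BP_Player stops overlapping it.
; On end overlap it loops LayerList, and InvertVisiblity sets each layer actor's hidden state to the opposite of LayerVisibility, which this graph never updates.
; The matching begin-overlap logic is disconnected.
; GetLayerActorVisibility, which reads the first layer's first actor, is never called here.
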(event Custom|SetLayerVisibility
  (for _array_element (Variables|Editable|GetLayerList)
    (CallFunction|InvertVisiblity _array_element)))

(event EventActorEndOverlap
  (params (OtherActor :type Actor%20Object%20Reference))
  (|CallParentFunction OtherActor)
  (Utilities|CheckTargetClass OtherActor "/Game/Blueprints/BP_Player.BP_Player_C"
    (:true
      (CallFunction|SetLayerVisibility))))

(event EventActorBeginOverlap
  (params (OtherActor :type Actor%20Object%20Reference)))

(fn ConstructionScript
  (|CallParentFunction))

(fn InvertVisiblity
  (params (ActorLayer :type Actor%20Layer%20Structure%20%28by%20ref%29))
  (bind _returnvalue (Class|LayersBlueprintLibrary|GetActors ActorLayer))
  (for _array_element _returnvalue
    (Rendering|SetActorHiddenInGame _array_element (not (Variables|Editable|GetLayerVisibility)))))

(fn GetLayerActorVisibility
  (bind _returnvalue (Class|LayersBlueprintLibrary|GetActors (Utilities|Array|Get(acopy) (Variables|Editable|GetLayerList))))
  (return (not (Variables|/Script/Engine.Actor|GetbHidden (Utilities|Array|Get(acopy) _returnvalue)))))