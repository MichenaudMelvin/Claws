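; BP_Bandage is an interactable bandage pickup placed in the world.
; Its construction script applies the Mesh variable to the static mesh component, so the pickup's look is set by that variable.
; On Interact, it passes BandagesValues to the main player controller's AddBandages and then destroys itself.
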(event EventBeginPlay
  (|CallParentFunction) ; This node is disabled and will not be called.\nDrag off pins to build functionality.
)

(event Collision|EventActorBeginOverlap
  (params (OtherActor :type Actor%20Object%20Reference)))

(event EventTick
  (params (DeltaSeconds :type Float%20%28single-precision%29))
  (|CallParentFunction DeltaSeconds) ; This node is disabled and will not be called.\nDrag off pins to build functionality.
)

(event EventInteract
  (params (MainPlayerController :type BP%20PC%20Main%20Player%20Controller%20Object%20Reference))
  (Default|AddBandages MainPlayerController (Variables|Default|GetBandagesValues))
  (Actor|DestroyActor))

(fn ConstructionScript
  (|CallParentFunction)
  (Components|StaticMesh|SetStaticMesh (Variables|Default|GetStaticMesh) (Variables|Default|GetMesh)))