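; BP_DigiDoor is a puzzle door that opens when the correct code is entered on its digicode keypad.
; Interact simulates a left click through the player's WidgetInteraction component to press keys on the world-space widget, which reports entered codes through a bound event.
; CheckCode compares the code, then either opens the inherited door with success feedback or signals an error, triggering the alarm on the third try.
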(event EventInteract
  (params (MainPlayerController :type BP%20PC%20Main%20Player%20Controller%20Object%20Reference))
  (bind _bp_player (Variables|/Game/Blueprints/Managers/BP_PC_MainPlayerController.BP_PC_MainPlayerController_C|GetBP_Player MainPlayerController))
  (bind _widgetinteraction (Variables|/Game/Blueprints/BP_Player.BP_Player_C|GetWidgetInteraction _bp_player))
  (Class|WidgetInteractionComponent|PressPointerKey _widgetinteraction "LeftMouseButton")
  (Class|WidgetInteractionComponent|ReleasePointerKey _widgetinteraction "LeftMouseButton"))

(event EventBeginPlay
  (Variables|Default|SetTargetInteraction (Variables|Default|GetDigicodeWidgetComponent))
  (|CallParentFunction)
  (bind _aswbp_digicode (Utilities|Casting|CastToWBP_Digicode (UserInterface|GetUserWidgetObject (Variables|Default|GetDigicodeWidgetComponent))))
  (bind _output_get (Variables|Default|SetDigicodeWidget _aswbp_digicode))
  (EventDispatchers|BindEventtoCodeEntered _output_get (EventDispatchers|CreateEvent :!event CheckCode)))

(fn ConstructionScript
  (|CallParentFunction))

(fn CheckCode
  (params (CodeEntered :type String) (Keypad :type WBP%20Digicode%20Object%20Reference))
  (Math|Integer|IncrementInt (Variables|Default|GetTries)
    (:%20%20
      (if (Utilities|Enum|Equal(Enum) CodeEntered (Variables|Default|GetCorrectCode))
        (CallFunction|OpenandCloseDoor (CallFunction|CallMainPlayerController))
        (Default|SuccessEvent Keypad (Transformation|GetWorldLocation (Variables|Default|GetDigicodeWidgetComponent)) self)
        (elif (== (Variables|Default|GetTries) 3)
          (Default|TriggerAlarm Keypad (Transformation|GetWorldLocation (Variables|Default|GetDigicodeWidgetComponent)) self)
          (Variables|Default|SetTries 0)
          (else
            (Default|ErrorEvent Keypad (Transformation|GetWorldLocation (Variables|Default|GetDigicodeWidgetComponent)) self)))))))