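; Puzzle generator actor meant to switch the spotlights in its LightList on and off, warning at BeginPlay when the list is empty.
; Interact is an empty stub, so the toggle logic never runs.
; That disconnected logic requires a held BP_Essence item, flips IsEnable and each spotlight's visibility, then calls a sound still missing its asset and reports a long-range noise event.
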(event EventBeginPlay
  (|CallParentFunction)
  (if (== (Utilities|Array|Length (Variables|Default|GetLightList)) 0)
    (Development|PrintString "Le générateur n'affecte aucunes lampes" true true "(R=1.000000,G=0.000000,B=0.000000,A=1.000000)" 9999999.0)))

(event EventInteract
  (params (MainPlayerController :type BP%20PC%20Main%20Player%20Controller%20Object%20Reference)))

(fn ConstructionScript
  (|CallParentFunction))