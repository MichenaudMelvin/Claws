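; BP_DigiDoor is a puzzle door actor with a keypad widget that checks an entered code against a correct one.
; On BeginPlay it gets the WBD_Digicode from its widget component and binds an event to CodeEntered.
; CheckCode compares the code, prints an opened or closed message and clears the keypad.
; The door is unfinished: player trigger overlaps do nothing and the unlock assignment never runs.
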(event OnComponentBeginOverlap(DoorTrigger)
  (params (OverlappedComponent :type Primitive%20Component%20Object%20Reference) (OtherActor :type Actor%20Object%20Reference) (OtherComp :type Primitive%20Component%20Object%20Reference) (OtherBodyIndex :type Integer) (bFromSweep :type Boolean) (SweepResult :type Hit%20Result%20Structure%20%28by%20ref%29))
  (if (== OtherActor (Game|GetPlayerCharacter 0))
    _))

(event OnComponentEndOverlap(DoorTrigger)
  (params (OverlappedComponent :type Primitive%20Component%20Object%20Reference) (OtherActor :type Actor%20Object%20Reference) (OtherComp :type Primitive%20Component%20Object%20Reference) (OtherBodyIndex :type Integer))
  (if (== (Game|GetPlayerCharacter 0) OtherActor)
    _))

(event Collision|EventActorBeginOverlap
  (params (OtherActor :type Actor%20Object%20Reference)))

(event EventTick
  (params (DeltaSeconds :type Float%20%28single-precision%29))
  (|CallParentFunction DeltaSeconds) ; This node is disabled and will not be called.\nDrag off pins to build functionality.
)

(event EventBeginPlay
  (bind _aswbd_digicode (Utilities|Casting|CastToWBD_Digicode (UserInterface|GetUserWidgetObject (Variables|Default|GetDigicodeWidget))))
  (bind _output_get (Variables|Default|SetAs%20WBD%20Digicode _aswbd_digicode))
  (EventDispatchers|BindEventtoCodeEntered _output_get (EventDispatchers|CreateEvent :!event CheckCode)))

(fn ConstructionScript
  (|CallParentFunction))

(fn CheckCode
  (params (CodeEntered :type String) (Keypad :type WBD%20Digicode%20Object%20Reference))
  (if (Utilities|Enum|Equal(Enum) CodeEntered (Variables|Default|GetCorrectCode))
    (Development|PrintString "Door Opened")
    (Variables|/Game/Blueprints/Puzzles/WBD_Digicode.WBD_Digicode_C|SetCurrentCode Keypad "")
    (else
      (Development|PrintString "Door Closed")
      (Variables|/Game/Blueprints/Puzzles/WBD_Digicode.WBD_Digicode_C|SetCurrentCode Keypad ""))))