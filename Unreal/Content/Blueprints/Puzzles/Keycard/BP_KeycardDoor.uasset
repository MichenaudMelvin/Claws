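; Keycard-locked door puzzle actor that opens its parent's interaction only to players holding the matching keycard.
; On BeginPlay it swaps the Door for the KeycardController in TargetInteraction, moving the interaction point to the controller.
; Interact searches the player's KeycardsList for DoorID and calls the parent Interact only on a match, printing each comparison to screen as debug output.
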(event EventBeginPlay
  (bind _targetinteraction (Variables|Default|GetTargetInteraction))
  (|CallParentFunction)
  (Utilities|Array|Add _targetinteraction (Variables|Default|GetKeycardController))
  (Utilities|Array|RemoveItem _targetinteraction (Variables|Default|GetDoor)))

(event EventInteract
  (params (MainPlayerController :type BP%20PC%20Main%20Player%20Controller%20Object%20Reference))
  (if (CallFunction|CheckKeycardID (Variables|/Game/Blueprints/BP_Player.BP_Player_C|GetKeycardsList (Variables|/Game/Blueprints/Managers/BP_PC_MainPlayerController.BP_PC_MainPlayerController_C|GetBP_Player MainPlayerController)))
    (|CallParentFunction MainPlayerController)))

(fn ConstructionScript
  (|CallParentFunction))

(fn CheckKeycardID
  (params (Array :type Array%20of%20Integers))
  (for _array_element Array
    (Development|PrintString (Utilities|String|ToString(Boolean) (== _array_element (Variables|Default|GetDoorID))))
    (if (== _array_element (Variables|Default|GetDoorID))
      (return true)))
  (return false))