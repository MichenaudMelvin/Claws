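; BP_Keycard is an interactable keycard pickup for the puzzle system.
; On interact it adds its ID to the player's KeycardsList and copies that list into the current save data.
; It then shows a timed story tip through the player controller's tip widget, with hardcoded text about director Sidwell Friedman, and destroys itself.
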(event EventInteract
  (params (MainPlayerController :type BP%20PC%20Main%20Player%20Controller%20Object%20Reference))
  (bind _bp_player (Variables|/Game/Blueprints/Managers/BP_PC_MainPlayerController.BP_PC_MainPlayerController_C|GetBP_Player MainPlayerController))
  (Utilities|Array|Add (Variables|/Game/Blueprints/BP_Player.BP_Player_C|GetKeycardsList _bp_player) (Variables|Default|GetID))
  (CallFunction|SetKeycardListonSave _bp_player)
  (Default|ShowSingleTip (Variables|/Game/Blueprints/Managers/BP_PC_MainPlayerController.BP_PC_MainPlayerController_C|GetTipWidget MainPlayerController) (Utilities|Struct|MakeSTRUCT_Tip "Sidwell Friedman ? So this guy was the director... scumbag." 5.5))
  (Actor|DestroyActor))

(fn ConstructionScript
  (|CallParentFunction))

(fn SetKeycardListonSave
  (params (BP_Player :type BP%20Player%20Object%20Reference))
  (Variables|/Game/Blueprints/Checkpoints/BP_SavedData.BP_SavedData_C|SetKeycardList (CallFunction|CallCurrentSaveData) (Variables|/Game/Blueprints/BP_Player.BP_Player_C|GetKeycardsList BP_Player)))