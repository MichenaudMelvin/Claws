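; BP_Item is a base interactable item with an empty Interact event and feedback events that outline its target components and show the E key prompt.
; Target components default to the static mesh when none are set.
; An interaction radius increments or decrements the player controller's nearby-item count, animating the pointer widget on first entry and last exit.
; While visible, the key text rotates each tick to face the camera.
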(event OnComponentBeginOverlap(InteractionRadius)
  (params (OverlappedComponent :type Primitive%20Component%20Object%20Reference) (OtherActor :type Actor%20Object%20Reference) (OtherComp :type Primitive%20Component%20Object%20Reference) (OtherBodyIndex :type Integer) (bFromSweep :type Boolean) (SweepResult :type Hit%20Result%20Structure%20%28by%20ref%29))
  (CallFunction|EnterInteractionRadius OtherActor))

(event OnComponentEndOverlap(InteractionRadius)
  (params (OverlappedComponent :type Primitive%20Component%20Object%20Reference) (OtherActor :type Actor%20Object%20Reference) (OtherComp :type Primitive%20Component%20Object%20Reference) (OtherBodyIndex :type Integer))
  (CallFunction|ExitInteractionRadius OtherActor))

(event Custom|EnterInteractionRadius
  (params (OtherActor :type Actor%20Object%20Reference))
  (Utilities|CheckTargetClass OtherActor "/Game/Blueprints/BP_Player.BP_Player_C"
    (:true
      (bind _result (Math|Integer|IncrementInt (Variables|/Game/Blueprints/Managers/BP_PC_MainPlayerController.BP_PC_MainPlayerController_C|GetInItemsSphere (CallFunction|CallMainPlayerController)))
        (:%20%20
          (if (== _result 1)
            (Default|PointeurAnimation (Variables|/Game/Blueprints/Managers/BP_PC_MainPlayerController.BP_PC_MainPlayerController_C|GetPointerWidget (CallFunction|CallMainPlayerController)) "Forward")))))))

(event Custom|ExitInteractionRadius
  (params (OtherActor :type Actor%20Object%20Reference))
  (bind _mainplayercontroller (CallFunction|CallMainPlayerController))
  (if (and (.ReturnValue (Utilities|CheckTargetClassPure OtherActor "/Game/Blueprints/BP_Player.BP_Player_C")) (Utilities|IsValid _mainplayercontroller))
    (bind _output_get (Variables|/Game/Blueprints/Managers/BP_PC_MainPlayerController.BP_PC_MainPlayerController_C|SetInItemsSphere _mainplayercontroller (Math|Integer|Clamp(Integer) (- (Variables|/Game/Blueprints/Managers/BP_PC_MainPlayerController.BP_PC_MainPlayerController_C|GetInItemsSphere _mainplayercontroller) 1) 0 2147483647)))
    (if (== _output_get 0)
      (Default|PointeurAnimation (Variables|/Game/Blueprints/Managers/BP_PC_MainPlayerController.BP_PC_MainPlayerController_C|GetPointerWidget (CallFunction|CallMainPlayerController)) "Reverse"))))

(event EventBeginPlay
  (Utilities|IsArrayNull (Variables|Appearance|GetTargetInteraction)
    (:true
      (Utilities|Array|Add (Variables|Appearance|GetTargetInteraction) (Variables|Default|GetStaticMesh)))
    (:false
      (CallFunction|OutlineActor false (Variables|Default|GetStaticMesh))))
  (Variables|Default|SetInteractionKey "E")
  (for _array_element (Variables|Appearance|GetTargetInteraction)
    (CallFunction|OutlineActor false _array_element))
  (Rendering|SetVisibility (Variables|Default|GetInputNameText) false true))

(event Input|ActionEvents|InputActionInteract
  (params (Key :type Key%20Structure :default "None")))

(event EventTick
  (params (DeltaSeconds :type Float%20%28single-precision%29))
  (Appearance|BillboardText))

(event EventInteract
  (params (MainPlayerController :type BP%20PC%20Main%20Player%20Controller%20Object%20Reference)))

(event EventFeedbackCanInteract
  (Rendering|SetVisibility (Variables|Default|GetInputNameText) true true)
  (Rendering|Components|TextRender|SetText (Variables|Default|GetInputNameText) (Class|KismetInputLibrary|KeyGetDisplayName (Variables|Default|GetInteractionKey)))
  (for _array_element (Variables|Appearance|GetTargetInteraction)
    (CallFunction|OutlineActor true _array_element)))

(event EventFeedbackStopCanInteract
  (Rendering|SetVisibility (Variables|Default|GetInputNameText) false true)
  (for _array_element (Variables|Appearance|GetTargetInteraction)
    (CallFunction|OutlineActor false _array_element)))

(fn ConstructionScript)

(fn BillboardText
  (if (Rendering|IsVisible (Variables|Default|GetInputNameText))
    (Transformation|SetWorldRotation (Variables|Default|GetInputNameText) (Math|Rotator|FindLookatRotation (Transformation|GetActorLocation) (Transformation|GetActorLocation (Game|GetPlayerCameraManager 0))) false false)))