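; Procedural scatter actor that builds a clamped number of BP_ModularMesh child actors from ModularMeshClass.
; The construction script assigns each a MeshList mesh using a seeded random stream, with relative transforms from RandomTransform.
; RandomTransform contains seeded XY, yaw and scale math, but that node appears unconnected.
; If AreObjectLaunchables is set, BeginPlay spawns BP_LaunchableObject copies with matching meshes and transforms, then destroys itself.
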(event EventBeginPlay
  (if (Variables|Editable|GetAreObjectLaunchables)
    (for _array_element (Variables|Default|GetElementList)
      (bind _returnvalue (Game|SpawnActorfromClass "/Game/Blueprints/LaunchableObjects/BP_LaunchableObject.BP_LaunchableObject_C" (Transformation|GetWorldTransform _array_element) "Undefined" 0 0))
      (bind _asbp_modular_mesh (Utilities|Casting|CastToBP_ModularMesh (Variables|/Script/Engine.ChildActorComponent|GetChildActor _array_element)))
      (Components|StaticMesh|SetStaticMesh (Variables|/Game/Blueprints/AbstactClasses/BP_Item.BP_Item_C|GetStaticMesh _returnvalue) (Variables|/Script/Engine.StaticMeshComponent|GetStaticMesh (Variables|/Game/Blueprints/AbstactClasses/BP_ModularMesh.BP_ModularMesh_C|GetModularMesh _asbp_modular_mesh))))
    (Actor|DestroyActor)))

(fn ConstructionScript
  (bind _meshlist (Variables|Editable|GetMeshList))
  (Utilities|Array|Clear (Variables|Default|GetElementList))
  (for _index (range 0 (- (Math|Integer|Clamp(Integer) (Variables|Editable|GetObjectsNumber) 1 (Variables|Editable|GetMaxObjectsNumber)) 1))
    (bind _returnvalue (AddComponent|AddChildActorComponent self false (|RandomTransform)))
    (Utilities|Array|Add (Variables|Default|GetElementList) _returnvalue))
  (for _array_element (Variables|Default|GetElementList)
    (ChildActorComponent|SetChildActorClass _array_element (Variables|Editable|GetModularMeshClass))
    (bind _asbp_modular_mesh (Utilities|Casting|CastToBP_ModularMesh (Variables|/Script/Engine.ChildActorComponent|GetChildActor _array_element)))
    (Components|StaticMesh|SetStaticMesh (Variables|/Game/Blueprints/AbstactClasses/BP_ModularMesh.BP_ModularMesh_C|GetModularMesh _asbp_modular_mesh) (Utilities|Array|Get(acopy) _meshlist (Math|Random|RandomIntegerinRangefromStream 0 (Utilities|Array|LastIndex _meshlist) (Variables|Editable|GetStream))))))

(fn RandomFloat
  (params (Float :type Float%20%28single-precision%29))
  (return (Math|Random|RandomFloatinRangefromStream (* -1 Float) Float (Variables|Editable|GetStream))))