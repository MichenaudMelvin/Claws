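; BP_EventTrigger is a trigger actor, filed as an abstract class, that reacts to the player entering and leaving its overlap area.
; Player entries and exits increment separate counters, and other actors are filtered out by a class check.
; Each entry also calls CancelEvents, which destroys every actor in CancelEventList.
; The construction script sets in-game visibility of the actor and its collision component from VisibleInGame.
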(event Collision|EventActorBeginOverlap
  (params (OtherActor :type Actor%20Object%20Reference))
  (Utilities|CheckTargetClass OtherActor "/Game/Blueprints/BP_Player.BP_Player_C"
    (:true
      (Math|Integer|IncrementInt (Variables|Default|GetEnterTriggerNumber)
        (:%20%20
          (CallFunction|CancelEvents))))))

(event Collision|EventActorEndOverlap
  (params (OtherActor :type Actor%20Object%20Reference))
  (Utilities|CheckTargetClass OtherActor "/Game/Blueprints/BP_Player.BP_Player_C"
    (:true
      (Math|Integer|IncrementInt (Variables|Default|GetExitTriggernumber)))))

(fn ConstructionScript
  (bind _visibleingame (Variables|Editable|GetVisibleInGame))
  (bind _returnvalue (not _visibleingame))
  (Rendering|SetActorHiddenInGame self _returnvalue)
  (Development|SetHiddeninGame (Variables|Default|GetCollisionComponent) _returnvalue true))

(fn CancelEvents
  (for _array_element (Variables|Editable|GetCancelEventList)
    (Actor|DestroyActor _array_element)))